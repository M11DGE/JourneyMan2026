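; BP_HailCloudManager is a trigger-volume actor that drives a set of hail clouds while its box is overlapped.
; Begin overlap starts or resumes a fast looping timer and end overlap pauses it, with no filter on the overlapping actor.
; Each cycle calls SpawnCloud on every ManagedClouds key with its melt time, delay and ice shape, then waits out a shared cooldown.
; The construction script applies the box extent and offset.
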(event `SpawnRoutine`
  (bind _managedclouds (`self.ManagedClouds`))
  (if (not (`self.bIsOnCoolDown`))
    (bind _keys (`BlueprintMapLibrary.Map_Keys` _managedclouds))
    (for _array_element _keys
      (bind (_initalspawndelay _icemelttime _iceshape) (break `/Game/_Project/Blueprints/_Core/Structures/F_HailCloud` (`BlueprintMapLibrary.Map_Find` _managedclouds _array_element)))
      (`/Game/_Project/Blueprints/BP_HailCloud.SpawnCloud` _array_element _icemelttime _initalspawndelay _iceshape))
    (set `self.bIsOnCoolDown` true)
    (`KismetSystemLibrary.Delay` (`self.CycleCooldown`))
    (set `self.bIsOnCoolDown` false)))

(event `StartSpawning`
  (if (`KismetSystemLibrary.K2_IsValidTimerHandle` (`self.TriggerHailCloudSpawn`))
    (`KismetSystemLibrary.K2_UnPauseTimerHandle` (`self.TriggerHailCloudSpawn`))
    (else
      (bind _returnvalue (`KismetSystemLibrary.K2_SetTimerDelegate` (delegate `SpawnRoutine`) 0.05 true true))
      (set `self.TriggerHailCloudSpawn` _returnvalue))))

(event `StopSpawning`
  (`KismetSystemLibrary.K2_PauseTimerHandle` (`self.TriggerHailCloudSpawn`)))

(event `self.Box.OnComponentBeginOverlap`
  (params (OverlappedComponent :type "PrimitiveComponent Object Reference") (OtherActor :type "Actor Object Reference") (OtherComp :type "PrimitiveComponent Object Reference") (OtherBodyIndex :type Integer) (bFromSweep :type Boolean) (SweepResult :type "HitResult Structure (by ref)"))
  (`self.StartSpawning`))

(event `self.Box.OnComponentEndOverlap`
  (params (OverlappedComponent :type "PrimitiveComponent Object Reference") (OtherActor :type "Actor Object Reference") (OtherComp :type "PrimitiveComponent Object Reference") (OtherBodyIndex :type Integer))
  (`self.StopSpawning`))

(fn `UserConstructionScript`
  (bind _box (`self.Box`))
  (`BoxComponent.SetBoxExtent` _box (`self.In Box Extent`) true)
  (`SceneComponent.K2_SetRelativeLocation` _box (`self.BoxOffset`) false false))