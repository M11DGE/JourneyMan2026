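; BP_LightCrystal_1 is an environment crystal prop pairing a static mesh with a point light in a shared, configurable colour.
; The Construction Script multiplies light intensity and source radius by the averaged X/Y world scale, and source length by Z, truncating scales to integers.
; It also applies the colour to the light and to the CrystalColor parameter of a dynamic material instance.
; The event graph holds no active logic.
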(fn `UserConstructionScript`
  (bind _pointlight (`self.PointLight`))
  (bind _staticmesh (`self.StaticMesh`))
  (bind _colour (`self.Colour`))
  (bind (_returnvalue_x _returnvalue_y _returnvalue_z) (`KismetMathLibrary.BreakVector` (`SceneComponent.K2_GetComponentScale` (`self.DefaultSceneRoot`))))
  (bind _averagevalue (`KismetMathLibrary.AverageOfIntArray` (`|MakeArray` (`KismetMathLibrary.FTrunc` _returnvalue_x) (`KismetMathLibrary.FTrunc` _returnvalue_y))))
  (`LightComponent.SetIntensity` _pointlight (* (`LightComponentBase.Intensity` _pointlight) _averagevalue))
  (`PointLightComponent.SetSourceLength` _pointlight (* (`PointLightComponent.SourceLength` _pointlight) (`KismetMathLibrary.FTrunc` _returnvalue_z)))
  (`PointLightComponent.SetSourceRadius` _pointlight (* (`PointLightComponent.SourceRadius` _pointlight) _averagevalue))
  (bind _returnvalue (`PrimitiveComponent.CreateDynamicMaterialInstance` _staticmesh 0 (`PrimitiveComponent.GetMaterial` _staticmesh 0) "None"))
  (`MaterialInstanceDynamic.SetVectorParameterValue` _returnvalue "CrystalColor" _colour)
  (`LightComponent.SetLightColor` (`self.PointLight`) _colour true))