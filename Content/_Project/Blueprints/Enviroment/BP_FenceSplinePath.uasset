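; Fence path actor that builds a collidable fence along an editable spline in its construction script.
; It divides spline length by the X-bounds length of MeshtoWrap and adds one spline mesh component per segment.
; The first segment always uses SM_Fence_Full, and the rest use MeshtoWrap.
; GetSplineInfoAtIndex supplies segment endpoints by distance along the spline, with tangents clamped to mesh length.
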(fn `UserConstructionScript`
  (bind (_tangent _location) (`self.GetSplineInfoAtIndex` 1))
  (bind (_tangent_2 _location_2) (`self.GetSplineInfoAtIndex` 0))
  (bind _output_get (set `self.MeshLength` (* (.x (`.BoxExtent` (`KismetMathLibrary.BreakBoxSphereBounds` (`StaticMesh.GetBounds` (`self.MeshtoWrap`))))) 2.0)))
  (bind _output_get_2 (set `self.NumberofInstances` (`KismetMathLibrary.FCeil` (/ (`SplineComponent.GetSplineLength` (`self.Spline`)) _output_get))))
  (`|ExecutionSequence`
    (:`then_0`
      (bind _returnvalue (`AddComponent|NODE_AddSplineMeshComponent-7` :`RelativeTransform` (`KismetMathLibrary.MakeTransform` (0.0 0.0 0.0) (struct) (1.5 1.5 1.5))))
      (`PrimitiveComponent.SetCollisionEnabled` _returnvalue "QueryAndPhysics")
      (`StaticMeshComponent.SetStaticMesh` _returnvalue "/Game/_Project/Art/Meshes/Decorative/Fences/SM_Fence_Full.SM_Fence_Full")
      (`SplineMeshComponent.SetStartAndEnd` _returnvalue _location_2 _tangent_2 _location _tangent true))
    (:`then_1`
      (for _index (range 2 (+ _output_get_2 1))
        (bind _returnvalue_2 (`AddComponent|NODE_AddSplineMeshComponent-0` :`RelativeTransform` (`KismetMathLibrary.MakeTransform` (0.0 0.0 0.0) (struct) (1.5 1.5 1.5))))
        (`PrimitiveComponent.SetCollisionEnabled` _returnvalue_2 "QueryAndPhysics")
        (`StaticMeshComponent.SetStaticMesh` _returnvalue_2 (`self.MeshtoWrap`))
        (bind (_tangent_3 _location_3) (`self.GetSplineInfoAtIndex` (- _index 1)))
        (bind (_tangent_4 _location_4) (`self.GetSplineInfoAtIndex` _index))
        (`SplineMeshComponent.SetStartAndEnd` _returnvalue_2 _location_3 _tangent_3 _location_4 _tangent_4 true)))))