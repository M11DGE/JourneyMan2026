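; BP_EventTrigger is a one-shot trigger volume that fires a named string event on the GM_AstorBot game mode.
; The first overlap on CollisionBox, with no filter on the overlapping actor, passes EventString to CallStringEvent and destroys the trigger.
; If EventString is empty, it prints a warning naming the actor and stays in the level, spent by its DoOnce.
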(event `self.CollisionBox.OnComponentBeginOverlap`
  (params (OverlappedComponent :type "PrimitiveComponent Object Reference") (OtherActor :type "Actor Object Reference") (OtherComp :type "PrimitiveComponent Object Reference") (OtherBodyIndex :type Integer) (bFromSweep :type Boolean) (SweepResult :type "HitResult Structure (by ref)"))
  (`/Engine/EditorBlueprintResources/StandardMacros.DoOnce` false
    (:`Completed`
      (if (`KismetStringLibrary.IsEmpty` (`self.EventString`))
        (`KismetSystemLibrary.PrintString` (`KismetStringLibrary.Concat_StrStr` "Event string not set for " (`KismetSystemLibrary.GetDisplayName` self)))
        (else
          (`/Game/_Project/Blueprints/GM_AstorBot.StringEvent` (cast `/Game/_Project/Blueprints/GM_AstorBot` (`GameplayStatics.GetGameMode`) :!pure true) (`self.EventString`))
          (`self.K2_DestroyActor`))))))

(fn `UserConstructionScript`)