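; Enemy spawner that handles the respawn of a single assigned enemy rather than spawning new actors.
; On BeginPlay it binds to the death event of EnemyToWatch, or prints a warning if none is set.
; When that enemy dies, it waits DelayBeforeRespawn, then switches the enemy's AI state to trigger the respawn, provided it is still in the expected state.
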(event `EnemyDied`
  (`KismetSystemLibrary.Delay` (`self.DelayBeforeRespawn`))
  (if (`|EnumEquality` (`/Game/_Project/Blueprints/Enemy/BP_EnemyPawn.AI_State` (`self.EnemyToWatch`)) "NewEnumerator5")
    (`/Game/_Project/Blueprints/Enemy/BP_EnemyPawn.SetAIState` (`self.EnemyToWatch`) "NewEnumerator6")))

(event `self.ReceiveBeginPlay`
  (`/Engine/EditorBlueprintResources/StandardMacros.IsValid` (`self.EnemyToWatch`)
    (:`Is Valid`
      (add `/Game/_Project/Blueprints/Enemy/BP_EnemyPawn.AIDie` (`self.EnemyToWatch`) (delegate `EnemyDied`)))
    (:`Is Not Valid`
      (`KismetSystemLibrary.PrintString` (`KismetStringLibrary.Concat_StrStr` (`KismetSystemLibrary.GetDisplayName` self) " EnemyToWatch not set")))))

(fn `UserConstructionScript`)