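; BP_MeltableTwinkle is an environment actor that shows a box-shaped Niagara flare effect, likely marking a meltable wall.
; On BeginPlay it sizes both the Niagara box and a debug box component from the BoxSize variable, doubling it for the effect.
; When WallMelted fires, it deactivates the effect and destroys itself once the system finishes, letting remaining particles fade out.
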(event `self.ReceiveBeginPlay`
  (bind _boxsize (`self.BoxSize`))
  (`NiagaraComponent.SetVariableVec3` (`self.NS_FlareBox`) "Box Size" (* _boxsize 2.0))
  (`BoxComponent.SetBoxExtent` (`self.DebugBox`) _boxsize false))

(event `WallMelted`
  (bind _ns_flarebox (`self.NS_FlareBox`))
  (add `NiagaraComponent.OnSystemFinished` _ns_flarebox (delegate `SystemFinished`))
  (`ActorComponent.Deactivate` _ns_flarebox))

(event `SystemFinished`
  (params (PSystem :type "NiagaraComponent Object Reference"))
  (`self.K2_DestroyActor`))

(fn `UserConstructionScript`)