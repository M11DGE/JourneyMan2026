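; BP_EnemyWatcher is an environment Blueprint that tracks a list of enemies and signals when all are destroyed.
; On BeginPlay it binds EnemyDestroyed to the AI death event of each entry in EnemiesToWatch.
; Each death triggers a rescan of every enemy's AIState against one enum value.
; When all match, it calls the AllEnemiesDestroyed dispatcher, letting other objects react without polling.
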(event `self.ReceiveBeginPlay`
  (for _array_element (`self.EnemiesToWatch`)
    (add `/Game/Enemy/BP_EnemyPawn.AIDie` _array_element (delegate `EnemyDestroyed`))))

(event `EnemyDestroyed`
  (set `self.bAllEnemiesDestroyed` true)
  (for _array_element (`self.EnemiesToWatch`)
    (if (not (`|EnumEquality` (`/Game/Enemy/BP_EnemyPawn.AI_State` _array_element) "NewEnumerator5"))
      (set `self.bAllEnemiesDestroyed` false)))
  (if (`self.bAllEnemiesDestroyed`)
    (`self.AllEnemiesDestroyed`)))

(fn `UserConstructionScript`)