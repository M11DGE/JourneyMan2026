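; BP_EndFlag is a level goal flag that triggers the player's win when they stand inside its end trigger.
; On overlap it stores the player and starts a per-frame looping timer that waits until the character is no longer falling.
; Once grounded, a DoOnce calls CallPlayerWin on GM_AstorBot and spawns a win Niagara effect at the flag.
; Leaving the trigger clears the player reference, though the timer keeps running.
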(event `self.EndPointTrigger.OnComponentBeginOverlap`
  (params (OverlappedComponent :type "PrimitiveComponent Object Reference") (OtherActor :type "Actor Object Reference") (OtherComp :type "PrimitiveComponent Object Reference") (OtherBodyIndex :type Integer) (bFromSweep :type Boolean) (SweepResult :type "HitResult Structure (by ref)"))
  (bind _asbp_player (cast `/Game/_Project/Blueprints/Characters/Player/BP_Player` OtherActor))
  (set `self.As BP Player` _asbp_player)
  (bind _returnvalue (`KismetSystemLibrary.K2_SetTimerDelegate` (delegate `CheckPlayerOnFloor`) 0.016667 true))
  (set `self.PlayerCheckFloorTimer` _returnvalue))

(event `self.EndPointTrigger.OnComponentEndOverlap`
  (params (OverlappedComponent :type "PrimitiveComponent Object Reference") (OtherActor :type "Actor Object Reference") (OtherComp :type "PrimitiveComponent Object Reference") (OtherBodyIndex :type Integer))
  (cast `/Game/_Project/Blueprints/Characters/Player/BP_Player` OtherActor)
  (set `self.As BP Player` null))

(event `CheckPlayerOnFloor`
  (bind _as_bp_player (`self.As BP Player`))
  (`/Engine/EditorBlueprintResources/StandardMacros.IsValid` _as_bp_player
    (:`Is Valid`
      (if (not (`NavMovementComponent.IsFalling` (`Character.CharacterMovement` _as_bp_player)))
        (`/Engine/EditorBlueprintResources/StandardMacros.DoOnce` false
          (:`Completed`
            (`/Game/_Project/Blueprints/GM_AstorBot.PlayerWin` (cast `/Game/_Project/Blueprints/GM_AstorBot` (`GameplayStatics.GetGameMode`) :!pure true))
            (`NiagaraFunctionLibrary.SpawnSystemAtLocation` "/Game/_Project/Art/Particles/AfterWin/NS_WinSpawn.NS_WinSpawn" (`self.K2_GetActorLocation`))
            (`KismetSystemLibrary.PrintString` "PlayerWin")))))))

(fn `UserConstructionScript`)