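; BP_Meltable is an environment actor that shrinks as it heats up and destroys itself once fully melted.
; Positive temperature changes from its temperature component set a target scale, reducing the starting scale linearly to zero at MaxHeat.
; Each change restarts a timeline that lerps the mesh from its current scale, destroying the actor if it finishes at zero.
; The construction script applies the configurable mesh and material.
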(event `self.ReceiveBeginPlay`
  (set `self.StartingScale` (`SceneComponent.RelativeScale3D` (`self.StaticMesh`))))

(event `self.AC_TemperatureComponent.CurrentTemperatureChanged`
  (params (CurrentTemperature :type Integer))
  (bind _maxheat (`/Game/_Project/Blueprints/Components/Temperature/AC_TemperatureComponent.MaxHeat` (`self.AC_TemperatureComponent`)))
  (if (> CurrentTemperature 0)
    (set `self.DesiredScale` (* (`self.StartingScale`) (/ (- _maxheat CurrentTemperature) _maxheat)))
    (if true
      (set `self.TimeLineStartScale` (`SceneComponent.RelativeScale3D` (`self.StaticMesh`)))
      (bind (_direction _newtrack_0) (`Timeline|Timeline` :!via `PlayFromStart`)
        (:`Update`
          (`SceneComponent.SetRelativeScale3D` (`self.StaticMesh`) (`KismetMathLibrary.VLerp` (`self.TimeLineStartScale`) (`self.DesiredScale`) _newtrack_0)))
        (:`Finished`
          (if (== (`SceneComponent.RelativeScale3D` (`self.StaticMesh`)) (0.0 0.0 0.0))
            (`self.K2_DestroyActor`)))))))

(fn `UserConstructionScript`
  (bind _staticmesh (`self.StaticMesh`))
  (`StaticMeshComponent.SetStaticMesh` _staticmesh (`self.ExportMesh`))
  (`PrimitiveComponent.SetMaterial` _staticmesh 0 (`self.InstancedMaterial`)))