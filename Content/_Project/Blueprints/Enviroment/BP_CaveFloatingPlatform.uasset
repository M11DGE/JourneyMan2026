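; BP_CaveFloatingPlatform is a cave platform that travels a looping route of preset locations, including one up a waterfall.
; BeginPlay places the mesh at the start and repeatedly runs the MovePlatform macro, which chains timed MoveComponentTo calls.
; If RedDoorOpen is true near the route's end, the platform glides back to the start.
; Otherwise it stops at another point, waits, teleports below the start and rises into place.
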(event `self.ReceiveBeginPlay`
  (`SceneComponent.K2_SetRelativeLocation` (`self.StaticMesh`) (`self.Location1`) false false)
  (for _ (range 3) :!label _label
    (`self.MovePlatform`
      (:`Completed`
        (goto _label))
      (:`Completed2`
        (goto _label)))))

(event `self.ReceiveTick`
  (params (DeltaSeconds :type "Float (single-precision)")))

(fn `UserConstructionScript`)