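; BP_HailCloud is an environment cloud actor that drops ice blocks when SpawnCloud is called.
; A looping or one-shot hover timeline offsets the cloud's height from BeginPlay until a delayed spawn stops it and animates sideways movement.
; It then spawns a BP_IceBlock below with the given melt time and shape, plays sound and Niagara burst, and animates cloud scale.
; The construction script can swap in an alternate mesh.
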(event `self.ReceiveBeginPlay`
  (bind (_originpos_x _originpos_y _originpos_z) (`KismetMathLibrary.BreakVector` (`self.OriginPos`)))
  (set `self.OriginPos` (`SceneComponent.RelativeLocation` (`self.HailCloud`)))
  (bind (_direction _newtrack_1) (`Timeline|Timeline_Hover`)
    (:`Update`
      (`SceneComponent.K2_SetRelativeLocation` (`self.HailCloud`) (`KismetMathLibrary.MakeVector` 0.0 0.0 (+ _originpos_z _newtrack_1)) false false))))

(event `SpawnCloud`
  (params (IceMeltTime :type "Float (double-precision)") (Delay :type "Float (double-precision)") (IceShape :type "/Game/_Project/Blueprints/_Core/Enums/E_PSButtons Enum" :default "NewEnumerator0"))
  (bind _returnvalue (`self.GetTransform`))
  (bind _hailcloud (`self.HailCloud`))
  (bind (_returnvalue_x _returnvalue_y _returnvalue_z) (`KismetMathLibrary.BreakVector` (`SceneComponent.K2_GetComponentLocation` (`self.HailCloud`))))
  (bind (_relativelocation_x _relativelocation_y _relativelocation_z) (`KismetMathLibrary.BreakVector` (`SceneComponent.RelativeLocation` _hailcloud)))
  (`KismetSystemLibrary.Delay` Delay)
  (`TimelineComponent.Stop` (`self.Timeline_Hover`))
  (bind (_direction _newtrack_0) (`Timeline|Timeline_PreSpawn` :!via `PlayFromStart`)
    (:`Update`
      (`SceneComponent.K2_SetRelativeLocation` _hailcloud (`KismetMathLibrary.MakeVector` _relativelocation_x _newtrack_0 _relativelocation_z) false false))
    (:`Finished`
      (bind _returnvalue_2 (`|SpawnActorFromClass` "/Game/_Project/Blueprints/Enviroment/BP_IceBlock.BP_IceBlock_C" (`KismetMathLibrary.MakeTransform` (`KismetMathLibrary.MakeVector` (.x (.location _returnvalue)) (.y (.location _returnvalue)) (- (.z (.location _returnvalue)) 130.0))) "Undefined" "MultiplyWithRoot" null IceMeltTime IceShape null))
      (`GameplayStatics.PlaySoundAtLocation` "/Game/_Project/Audio/SQ_IceBlockSpawn.SQ_IceBlockSpawn" (`self.K2_GetActorLocation` _returnvalue_2) (struct) 1.0 1.0 0.0 null null null null)
      (`NiagaraFunctionLibrary.SpawnSystemAtLocation` "/Game/_Project/Art/Particles/NS_IceDropBurst.NS_IceDropBurst" (`KismetMathLibrary.MakeVector` _returnvalue_x _returnvalue_y (- _returnvalue_z 10.0)))
      (bind (_direction_2 _newtrack_1) (`Timeline|Timeline_Spawn` :!via `PlayFromStart`)
        (:`Update`
          (`SceneComponent.SetRelativeScale3D` (`self.HailCloud`) (`KismetMathLibrary.MakeVector` _newtrack_1 _newtrack_1 _newtrack_1)))))))

(fn `UserConstructionScript`
  (`|ExecutionSequence`
    (:`then_0`
      (if (`self.UseAltMesh`)
        (`StaticMeshComponent.SetStaticMesh` (`self.HailCloud`) "/Game/_Project/Art/Meshes/Decorative/SM_HailCloud_2.SM_HailCloud_2")))))