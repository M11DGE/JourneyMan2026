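; Hail cloud manager that spawns its managed clouds in repeated cycles while its trigger box is overlapped.
; Box overlaps start or pause a looping timer that calls SpawnCloud on each cloud with its ice shape, melt time and initial delay, then waits out a cycle cooldown.
; The last entered of PointA or PointB selects forward or reverse cloud settings.
; The construction script sizes all three boxes.
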(event `SpawnRoutine`
  (bind _managedclouds (`self.ManagedClouds`))
  (if (not (`self.bIsOnCoolDown`))
    (bind _keys (`BlueprintMapLibrary.Map_Keys` _managedclouds))
    (if (`self.InsidePointA`)
      (for _array_element _keys
        (bind (_initalspawndelay _icemelttime _iceshape) (break `/Game/_Project/Blueprints/_Core/Structures/F_HailCloud` (`BlueprintMapLibrary.Map_Find` _managedclouds _array_element)))
        (`/Game/_Project/Blueprints/Enviroment/BP_HailCloud.SpawnCloud` _array_element _icemelttime _initalspawndelay _iceshape))
      (set `self.bIsOnCoolDown` true)
      (`KismetSystemLibrary.Delay` (`self.CycleCooldown`))
      (set `self.bIsOnCoolDown` false)
      (elif (`self.InsidePointB`)
        (for _array_element_2 _keys
          (bind (_initalspawndelay_2 _icemelttime_2 _iceshape_2) (break `/Game/_Project/Blueprints/_Core/Structures/F_HailCloud` (`BlueprintMapLibrary.Map_Find` (`self.Managed Clouds Reverse`) _array_element_2)))
          (`/Game/_Project/Blueprints/Enviroment/BP_HailCloud.SpawnCloud` _array_element_2 _icemelttime_2 _initalspawndelay_2 _iceshape_2))
        (set `self.bIsOnCoolDown` true)
        (`KismetSystemLibrary.Delay` (`self.CycleCooldown`))
        (set `self.bIsOnCoolDown` false)))))

(event `StartSpawning`
  (if (`KismetSystemLibrary.K2_IsValidTimerHandle` (`self.TriggerHailCloudSpawn`))
    (`KismetSystemLibrary.K2_UnPauseTimerHandle` (`self.TriggerHailCloudSpawn`))
    (else
      (bind _returnvalue (`KismetSystemLibrary.K2_SetTimerDelegate` (delegate `SpawnRoutine`) 0.05 true true))
      (set `self.TriggerHailCloudSpawn` _returnvalue))))

(event `StopSpawning`
  (`KismetSystemLibrary.K2_PauseTimerHandle` (`self.TriggerHailCloudSpawn`)))

(event `self.Box.OnComponentBeginOverlap`
  (params (OverlappedComponent :type "PrimitiveComponent Object Reference") (OtherActor :type "Actor Object Reference") (OtherComp :type "PrimitiveComponent Object Reference") (OtherBodyIndex :type Integer) (bFromSweep :type Boolean) (SweepResult :type "HitResult Structure (by ref)"))
  (`self.StartSpawning`))

(event `self.Box.OnComponentEndOverlap`
  (params (OverlappedComponent :type "PrimitiveComponent Object Reference") (OtherActor :type "Actor Object Reference") (OtherComp :type "PrimitiveComponent Object Reference") (OtherBodyIndex :type Integer))
  (`self.StopSpawning`))

(event `self.PointA.OnComponentBeginOverlap`
  (params (OverlappedComponent :type "PrimitiveComponent Object Reference") (OtherActor :type "Actor Object Reference") (OtherComp :type "PrimitiveComponent Object Reference") (OtherBodyIndex :type Integer) (bFromSweep :type Boolean) (SweepResult :type "HitResult Structure (by ref)"))
  (set `self.InsidePointB` false)
  (set `self.InsidePointA` true))

(event `self.PointA.OnComponentEndOverlap`
  (params (OverlappedComponent :type "PrimitiveComponent Object Reference") (OtherActor :type "Actor Object Reference") (OtherComp :type "PrimitiveComponent Object Reference") (OtherBodyIndex :type Integer)))

(event `self.PointB.OnComponentBeginOverlap`
  (params (OverlappedComponent :type "PrimitiveComponent Object Reference") (OtherActor :type "Actor Object Reference") (OtherComp :type "PrimitiveComponent Object Reference") (OtherBodyIndex :type Integer) (bFromSweep :type Boolean) (SweepResult :type "HitResult Structure (by ref)"))
  (set `self.InsidePointA` false)
  (set `self.InsidePointB` true))

(event `self.PointB.OnComponentEndOverlap`
  (params (OverlappedComponent :type "PrimitiveComponent Object Reference") (OtherActor :type "Actor Object Reference") (OtherComp :type "PrimitiveComponent Object Reference") (OtherBodyIndex :type Integer)))

(fn `UserConstructionScript`
  (bind _box (`self.Box`))
  (`BoxComponent.SetBoxExtent` _box (`self.In Box Extent`) true)
  (`SceneComponent.K2_SetRelativeLocation` _box (`self.BoxOffset`) false false)
  (`BoxComponent.SetBoxExtent` (`self.PointA`) (`self.In Point A Extent`) true)
  (`BoxComponent.SetBoxExtent` (`self.PointB`) (`self.In Point B Extent`) true))