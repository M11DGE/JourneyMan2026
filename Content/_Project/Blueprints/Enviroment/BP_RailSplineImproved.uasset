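; Rail spline actor that builds a segmented rail from spline meshes along its spline at construction time.
; The construction script derives the segment count from spline length and Mesh1's bounds, swapping in Mesh2 on every eighth segment.
; Segments have collision disabled and take endpoints from GetSplineInfoAtIndex, a helper with nodes for location and length-clamped tangent by distance.
; The event graph holds no logic.
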(fn `UserConstructionScript`
  (bind _output_get (set `self.MeshLength` (* (.x (`.BoxExtent` (`KismetMathLibrary.BreakBoxSphereBounds` (`StaticMesh.GetBounds` (`self.Mesh1`))))) 2.0)))
  (bind _output_get_2 (set `self.NumberofInstances` (`KismetMathLibrary.FCeil` (/ (`SplineComponent.GetSplineLength` (`self.Spline`)) _output_get))))
  (for _index (range 1 (+ _output_get_2 1))
    (bind _returnvalue (`AddComponent|NODE_AddSplineMeshComponent-0`))
    (`PrimitiveComponent.SetCollisionEnabled` _returnvalue "NoCollision")
    (if (> (mod _index 8) 0)
      (`StaticMeshComponent.SetStaticMesh` _returnvalue (`self.Mesh1`))
      (else
        (`StaticMeshComponent.SetStaticMesh` _returnvalue (`self.Mesh2`))))
    (bind (_location _tangent) (`self.GetSplineInfoAtIndex` (- _index 1)))
    (bind (_location_2 _tangent_2) (`self.GetSplineInfoAtIndex` _index))
    (`SplineMeshComponent.SetStartAndEnd` _returnvalue _location _tangent _location_2 _tangent_2 true)))