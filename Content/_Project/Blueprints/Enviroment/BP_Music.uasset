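; Level music actor that fades in an Intro track on play unless muted and swaps it for a Goal track when GM_AstroBot signals a player win.
; It sets the Intro's Index parameter to 1 after the SW sound's duration or when Intro audio finishes, if not muted.
; A ShadowFade parameter rises as a supplied distance approaches MinDistance.
; A one-shot FadeOut uses a timeline to lerp ShadowFade to zero.
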(event `self.ReceiveBeginPlay`
  (bind _bismute (`self.bIsMute`))
  (add `/Game/_Project/Blueprints/_Core/GM_AstroBot.PlayerWin` (cast `/Game/_Project/Blueprints/_Core/GM_AstroBot` (`GameplayStatics.GetGameMode`) :!pure true) (delegate `PlayerWin`))
  (if _bismute
    (`AudioComponent.Stop` (`self.Intro`))
    (else
      (`AudioComponent.FadeIn` (`self.Intro`) 5.0 1.0 0.0 "Linear")
      (`KismetSystemLibrary.Delay` (`SoundBase.Duration` (`self.SW`)))
      (if (not _bismute) :!label _label
        (`AudioComponent.SetIntParameter` (`self.Intro`) "Index" 1)))))

(event `PlayerWin`
  (`AudioComponent.Stop` (`self.Intro`))
  (`AudioComponent.Play` (`self.Goal`) 0.0))

(event `self.Intro.OnAudioFinished`
  (goto _label))

(event `FadeOut`
  (`/Engine/EditorBlueprintResources/StandardMacros.DoOnce` false
    (:`Completed`
      (set `self.FadeOutStartFade` (`self.LastFade`))
      (bind (_direction _newtrack_0) (`Timeline|Timeline` :!via `PlayFromStart`)
        (:`Update`
          (`AudioComponent.SetFloatParameter` (`self.Intro`) "ShadowFade" (`KismetMathLibrary.Lerp` (`self.FadeOutStartFade`) 0.0 _newtrack_0)))))))

(event `SetShadowFadeParam`
  (params (Distance :type "Float (double-precision)"))
  (bind _output_get (set `self.LastFade` (`KismetMathLibrary.MapRangeClamped` Distance (`self.MaxDistance`) (`self.MinDistance`) 0.0 1.0)))
  (`AudioComponent.SetFloatParameter` (`self.Intro`) "ShadowFade" _output_get))

(fn `UserConstructionScript`)