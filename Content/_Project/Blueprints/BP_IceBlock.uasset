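; BP_IceBlock is an ice block actor that melts away over a configurable lifetime.
; The construction script picks its mesh from Shape and caches its starting scale.
; On BeginPlay, a timer covers the full melt time, while a delayed timeline shrinks the mesh over the remaining portion using a runtime-assigned curve, normalized by its end value.
; When the timer fires, it broadcasts IceDestory and destroys the actor.
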(event `self.ReceiveBeginPlay`
  (bind _melttimeline (`self.MeltTimeline`))
  (bind _timeforfullmelt (`self.TimeForFullMelt`))
  (bind _floatcurve (`self.FloatCurve`))
  (bind _output_get (set `self.TimeForStartMelt` (* _timeforfullmelt (`self.PercentageBeforeStartMelt`))))
  (set `self.TimeToMelt` (- _timeforfullmelt _output_get))
  (`|ExecutionSequence`
    (:`then_0`
      (`KismetSystemLibrary.K2_SetTimerDelegate` (delegate `Melt`) _timeforfullmelt))
    (:`then_1`
      (`TimelineComponent.SetTimelineLength` _melttimeline (`self.TimeToMelt`))
      (`TimelineComponent.SetFloatCurve` _melttimeline _floatcurve "Alpha")
      (`KismetSystemLibrary.Delay` _output_get)
      (bind (_direction _alpha) (`Timeline|MeltTimeline`)
        (:`Update`
          (`SceneComponent.SetRelativeScale3D` (`self.IceBlock`) (`KismetMathLibrary.VLerp` (`self.IceBlockRelativeScale`) (0.0 0.0 0.0) (/ _alpha (`CurveFloat.GetFloatValue` _floatcurve (`self.TimeToMelt`))))))))))

(event `Melt`
  (`self.IceDestory` self)
  (`self.K2_DestroyActor`))

(fn `UserConstructionScript`
  (set `self.IceBlockRelativeScale` (`SceneComponent.RelativeScale3D` (`self.IceBlock`)))
  (switch `/Game/_Project/Blueprints/_Core/Enums/E_PSButtons` (`self.Shape`)
    (:`NewEnumerator0`
      (`StaticMeshComponent.SetStaticMesh` (`self.IceBlock`) "/Game/_Project/Art/Meshes/IceBlocks/SM_IceBlock_X.SM_IceBlock_X"))
    (:`NewEnumerator1`
      (`StaticMeshComponent.SetStaticMesh` (`self.IceBlock`) "/Game/_Project/Art/Meshes/IceBlocks/SM_IceBlock_Square.SM_IceBlock_Square"))
    (:`NewEnumerator2`
      (`StaticMeshComponent.SetStaticMesh` (`self.IceBlock`) "/Game/_Project/Art/Meshes/IceBlocks/SM_IceBlock_Triangle.SM_IceBlock_Triangle"))
    (:`NewEnumerator3`
      (`StaticMeshComponent.SetStaticMesh` (`self.IceBlock`) "/Game/_Project/Art/Meshes/IceBlocks/SM_IceBlock_Circle.SM_IceBlock_Circle"))))