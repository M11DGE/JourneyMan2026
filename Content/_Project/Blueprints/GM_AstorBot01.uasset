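; Game mode for an Astro Bot-style level that tracks coin and bot collection and drives both pickup HUD widgets.
; On BeginPlay it creates both widgets, numbers every BP_Co_Bot from its array index, and binds to its collected event.
; A collected bot's ID updates its icon in the bot widget, shown for two seconds.
; AddCoins accumulates the coin total and briefly shows the updated coin widget.
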(event `self.ReceiveBeginPlay`
  ; UI
  (`|ExecutionSequence`
    (:`then_0`
      (bind _returnvalue (`|CreateWidget` "/Game/_Project/UI/CoinCollect_UI.CoinCollect_UI_C"))
      (bind _output_get (set `self.Coin Collect UI` _returnvalue))
      (`UserWidget.AddToViewport` _output_get 0)
      (`Widget.SetVisibility` _output_get "Visible"))
    (:`then_1`
      (bind _returnvalue_2 (`|CreateWidget` "/Game/_Project/Blueprints/Co_Bot_UI.Co_Bot_UI_C"))
      (bind _output_get_2 (set `self.Co Bot UI` _returnvalue_2))
      (`UserWidget.AddToViewport` _output_get_2 0)
      (`Widget.SetVisibility` _output_get_2 "Hidden"))
    (:`then_2`
      ; Bot_Collect
      (bind _outactors (`GameplayStatics.GetAllActorsOfClass` "/Game/_Project/Blueprints/BP_Co_Bot.BP_Co_Bot_C"))
      (for (_array_element _array_index) _outactors
        (bind _asbp_co_bot (cast `/Game/_Project/Blueprints/BP_Co_Bot` _array_element))
        (set `/Game/_Project/Blueprints/BP_Co_Bot.UniqueID` (+ _array_index 1) _asbp_co_bot)
        (add `/Game/_Project/Blueprints/BP_Co_Bot.CoBotCollected` _asbp_co_bot (delegate `自定义事件`))))))

(event `自定义事件`
  (params (UniqueID :type Integer))
  ; Bot_Collect
  (bind _foundwidgets (`WidgetBlueprintLibrary.GetAllWidgetsOfClass` "/Game/_Project/Blueprints/Co_Bot_UI.Co_Bot_UI_C"))
  (bind _asco_bot_ui (cast `/Game/_Project/Blueprints/Co_Bot_UI` (`|GetArrayItem` _foundwidgets)))
  (`/Game/_Project/Blueprints/Co_Bot_UI.UpdateBotIcon` _asco_bot_ui UniqueID)
  (`Widget.SetVisibility` _asco_bot_ui "Visible")
  (`KismetSystemLibrary.Delay` 2.0)
  (`Widget.SetVisibility` _asco_bot_ui "Hidden")
  (switch `int` UniqueID))

(event `self.Add Coins`
  (params (CoinValue :type Integer))
  ; Coin_Collect
  (bind _output_get (set `self.CoinAmount` (+ (`self.CoinAmount`) CoinValue)))
  (`TextBlock.SetText` (`/Game/_Project/UI/CoinCollect_UI.CoinAmount` (`self.Coin Collect UI`)) (`|GenericToText` _output_get))
  (`Widget.SetVisibility` (`self.Coin Collect UI`) "Visible")
  (`KismetSystemLibrary.Delay` 2.0)
  (`Widget.SetVisibility` (`self.Coin Collect UI`) "Hidden"))

(fn `UserConstructionScript`)