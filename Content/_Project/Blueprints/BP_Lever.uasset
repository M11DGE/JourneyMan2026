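; BP_Lever is an interactable lever that sets two doors and changes pawn speed in a slow zone.
; A sphere overlap enables input, and F sets BlueDoor true and RedDoor false.
; It also sets SlowZone's SlowSpeed, applies it as MaxSpeed to overlapping pawns, then zeroes SlowSpeed after an in-loop delay, without reapplying it.
; An older door-toggle branch is left unconnected.
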(event `self.Sphere.OnComponentBeginOverlap`
  (params (OverlappedComponent :type "PrimitiveComponent Object Reference") (OtherActor :type "Actor Object Reference") (OtherComp :type "PrimitiveComponent Object Reference") (OtherBodyIndex :type Integer) (bFromSweep :type Boolean) (SweepResult :type "HitResult Structure (by ref)"))
  (`self.EnableInput` (`GameplayStatics.GetPlayerController` 0))
  (set `self.BPlayerInRange` true))

(event `Key|F`
  (params (Key :type "Key Structure"))
  (bind _slowzone (`self.SlowZone`))
  (:`Pressed`
    (if (`self.BPlayerInRange`)
      (`/Game/_Project/Blueprints/BP_DoubleDoor.SetDoorState` (`self.BlueDoor`) true)
      (`/Game/_Project/Blueprints/BP_DoubleDoor.SetDoorState` (`self.RedDoor`) false)
      (set `/Game/_Project/Blueprints/Minecraft/BP_SlowZone.SlowSpeed` 200.0 _slowzone)
      (for _array_element (`self.GetOverlappingActors` (`self.SlowZone`) "/Game/_Project/Blueprints/Minecraft/BP_MinecraftPawnNomarl.BP_MinecraftPawnNomarl_C")
        (bind _asbp_minecraft_pawn_nomarl (cast `/Game/_Project/Blueprints/Minecraft/BP_MinecraftPawnNomarl` _array_element))
        (set `FloatingPawnMovement.MaxSpeed` (`/Game/_Project/Blueprints/Minecraft/BP_SlowZone.SlowSpeed` _slowzone) (`/Game/_Project/Blueprints/Minecraft/BP_MinecraftPawnNomarl.FloatingPawnMovement` _asbp_minecraft_pawn_nomarl))
        (`KismetSystemLibrary.Delay` 10.0)
        (set `/Game/_Project/Blueprints/Minecraft/BP_SlowZone.SlowSpeed` 0.0 _slowzone)))))

(event `self.Sphere.OnComponentEndOverlap`
  (params (OverlappedComponent :type "PrimitiveComponent Object Reference") (OtherActor :type "Actor Object Reference") (OtherComp :type "PrimitiveComponent Object Reference") (OtherBodyIndex :type Integer))
  (`self.DisableInput` (`GameplayStatics.GetPlayerController` 0))
  (set `self.BPlayerInRange` false))

(fn `UserConstructionScript`)