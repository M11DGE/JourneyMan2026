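; BP_FriendBot is a collectable bot character that the player collects by attacking it.
; UniqueID selects its skeletal mesh in the construction script and the matching looping idle animation on BeginPlay, switching between Astrobot and SnowBoarder variants.
; When attacked, it reports its UniqueID to the game mode as a collectable message, plays a pickup sound at the player's location and destroys itself.
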(event `self.ReceiveBeginPlay`
  (`SkeletalMeshComponent.PlayAnimation` (`self.Co_Bot`) (select `int` (`self.UniqueID`) :`0` "/Game/_Project/Art/Characters/Player/Animations/Idle/AS_Astrobot_Idle.AS_Astrobot_Idle" :`1` "/Game/_Project/Art/Characters/Friends/SnowBoard/AS_SnowBoarder_Idle.AS_SnowBoarder_Idle" :`2` "/Game/_Project/Art/Characters/Player/Animations/Idle/AS_Astrobot_Idle.AS_Astrobot_Idle" :!type "AnimationAsset Object Reference") true))

(event `/Game/_Project/Blueprints/_Core/Interfaces/BPI_AttackReceiver.OnAttackReceived`
  (params (DamageAmount :type "Float (double-precision)") (KnockbackForce :type "Vector Structure") (Instigator :type "Actor Object Reference") (DamageType :type "/Game/_Project/Blueprints/_Core/Enums/E_DamageType Enum" :default "NewEnumerator0"))
  (message `/Game/_Project/Blueprints/_Core/Interfaces/BPI_Collectable.AddCollectable` (`GameplayStatics.GetGameMode`) "NewEnumerator1" (`self.UniqueID`))
  (`GameplayStatics.PlaySoundAtLocation` "/Game/_Project/Audio/Raw/MS_PuzzlePieceGet.MS_PuzzlePieceGet" (`self.K2_GetActorLocation` (`GameplayStatics.GetPlayerCharacter` 0)) (struct) 1.0 1.0 0.0 null null null null)
  (`self.K2_DestroyActor`))

(fn `UserConstructionScript`
  (`SkeletalMeshComponent.SetSkeletalMeshAsset` (`self.Co_Bot`) (select `int` (`self.UniqueID`) :`0` "/Game/_Project/Art/Characters/Player/Animations/SKM_Astrobot.SKM_Astrobot" :`1` "/Game/_Project/Art/Characters/Friends/SnowBoard/SKM_SnowBoarder_Master.SKM_SnowBoarder_Master" :`2` "/Game/_Project/Art/Characters/Player/Animations/SKM_Astrobot.SKM_Astrobot" :!type "SkeletalMesh Object Reference")))