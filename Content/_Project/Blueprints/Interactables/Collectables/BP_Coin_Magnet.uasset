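; BP_Coin_Magnet is a collectable coin that pops out on spawn and then flies to the player.
; BeginPlay launches the coin mesh with a random upward impulse, then after a short delay disables physics and starts the magnet.
; Tick then interpolates the mesh toward the player's location with VInterpTo.
; Overlap by BP_Player reports the coin to the game mode, plays pickup sound and Niagara effect, and destroys the actor.
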(event `self.CoinCollsion.OnComponentBeginOverlap`
  (params (OverlappedComponent :type "PrimitiveComponent Object Reference") (OtherActor :type "Actor Object Reference") (OtherComp :type "PrimitiveComponent Object Reference") (OtherBodyIndex :type Integer) (bFromSweep :type Boolean) (SweepResult :type "HitResult Structure (by ref)"))
  (bind _returnvalue (`self.K2_GetActorLocation` (`GameplayStatics.GetPlayerCharacter` 0)))
  (cast `/Game/_Project/Blueprints/Characters/Player/BP_Player` OtherActor)
  (message `/Game/_Project/Blueprints/_Core/Interfaces/BPI_Collectable.AddCollectable` (`GameplayStatics.GetGameMode`) "NewEnumerator0" 1)
  (`GameplayStatics.PlaySoundAtLocation` "/Game/_Project/Audio/SQ_Coin.SQ_Coin" _returnvalue (struct) 1.0 1.0 0.0 null null null null)
  (`NiagaraFunctionLibrary.SpawnSystemAtLocation` "/Game/_Project/Blueprints/Interactables/Collectables/NS_CoinCollection.NS_CoinCollection" _returnvalue)
  (`self.K2_DestroyActor`))

(event `self.ReceiveBeginPlay`
  (`PrimitiveComponent.AddImpulse` (`self.Coin_Mesh`) (* (`KismetMathLibrary.MakeVector` (* (.x (`KismetMathLibrary.RandomUnitVector`)) 0.2) (* (.y (`KismetMathLibrary.RandomUnitVector`)) 0.2) (+ (.z (`KismetMathLibrary.RandomUnitVector`)) 1.5)) 500.0) "None" true)
  (`KismetSystemLibrary.Delay` 1.0)
  (`PrimitiveComponent.SetSimulatePhysics` (`self.Coin_Mesh`) false)
  (set `self.TargetPlayer` (`GameplayStatics.GetPlayerCharacter` 0))
  (set `self.bStartMagnet` true))

(event `self.ReceiveTick`
  (params (DeltaSeconds :type "Float (single-precision)"))
  (if (`self.bStartMagnet`)
    (`SceneComponent.K2_SetWorldLocation` (`self.Coin_Mesh`) (`KismetMathLibrary.VInterpTo` (`SceneComponent.K2_GetComponentLocation` (`self.Coin_Mesh`)) (`self.K2_GetActorLocation` (`self.TargetPlayer`)) DeltaSeconds 10.0) false false)))

(fn `UserConstructionScript`)