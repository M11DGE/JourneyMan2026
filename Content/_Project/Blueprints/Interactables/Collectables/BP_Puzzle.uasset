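; BP_Puzzle is a collectable puzzle piece that the player picks up by touching it.
; BeginPlay caches the GM_AstroBot game mode.
; When BP_Player overlaps its sphere, it reports the pickup to the game mode as a collectable message carrying its UniqueNumber.
; It then plays the puzzle-piece sound at the player's location and destroys itself.
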(event `self.ReceiveBeginPlay`
  (bind _asgm_astro_bot (cast `/Game/_Project/Blueprints/_Core/GM_AstroBot` (`GameplayStatics.GetGameMode`)))
  (set `self.As GM Astor Bot` _asgm_astro_bot))

(event `self.Sphere1.OnComponentBeginOverlap`
  (params (OverlappedComponent :type "PrimitiveComponent Object Reference") (OtherActor :type "Actor Object Reference") (OtherComp :type "PrimitiveComponent Object Reference") (OtherBodyIndex :type Integer) (bFromSweep :type Boolean) (SweepResult :type "HitResult Structure (by ref)"))
  (cast `/Game/_Project/Blueprints/Characters/Player/BP_Player` OtherActor)
  (message `/Game/_Project/Blueprints/_Core/Interfaces/BPI_Collectable.AddCollectable` (`self.As GM Astor Bot`) "NewEnumerator2" (`self.Unique Number`))
  (`GameplayStatics.PlaySoundAtLocation` "/Game/_Project/Audio/Raw/MS_PuzzlePieceGet.MS_PuzzlePieceGet" (`self.K2_GetActorLocation` (`GameplayStatics.GetPlayerCharacter` 0)) (struct) 1.0 1.0 0.0 null null null null)
  (`self.K2_DestroyActor`))

(fn `UserConstructionScript`)