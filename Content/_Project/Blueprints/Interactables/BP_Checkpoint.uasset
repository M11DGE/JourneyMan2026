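; Checkpoint actor that activates once, when the player enters its configurable trigger volume or already overlaps it shortly after BeginPlay.
; Activation sends the respawn transform and checkpoint ID to the game mode.
; If the game mode accepts it as new, the light and hologram turn blue and a sound plays.
; Construction sets the hologram red using a color DataTable, and Tick rotates its pivot to face the player.
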(event `self.ReceiveBeginPlay`
  (bind _astroblue_color (break `/Game/_Project/Blueprints/_Core/Structures/F_Color` (`self.AstroBlue`)))
  (bind _astroblue_color_2 (break `/Game/_Project/Blueprints/_Core/Structures/F_Color` (`self.AstroBlue`)))
  (`KismetSystemLibrary.Delay` 0.1)
  (for _array_element (`PrimitiveComponent.GetOverlappingActors` (`self.TriggerVolume`) "/Game/_Project/Blueprints/Characters/Player/BP_Player.BP_Player_C")
    (if (== (`GameplayStatics.GetObjectClass` _array_element) "/Game/_Project/Blueprints/Characters/Player/BP_Player.BP_Player_C")
      (set `self.Condition` true)))
  (if (`self.Condition`)
    ; Checkpoint can only be activated once in lifetime
    (if (not (`self.bIsActivated`)) :!label _label
      (set `self.bIsActivated` true)
      (bind _bwasaccepted (message `/Game/_Project/Blueprints/_Core/Interfaces/BPI_CheckpointManager.UpdateActiveCheckpoint` (`GameplayStatics.GetGameMode`) (`SceneComponent.K2_GetComponentToWorld` (`self.RespawnDir`)) (`self.CheckpointID`)))
      ; Only changes visuals if checkpoint is new - not old/missed
      (if _bwasaccepted
        (`LightComponent.SetLightColor` (`self.CheckpointLightStatus`) (`KismetMathLibrary.Conv_ColorToLinearColor` _astroblue_color) true)
        (`GameplayStatics.PlaySoundAtLocation` null (`self.K2_GetActorLocation`) (struct) 1.0 1.0 0.0 null null null null)
        (`self.SetHologramColor` _astroblue_color_2)))))

(event `self.TriggerVolume.OnComponentBeginOverlap`
  (params (OverlappedComponent :type "PrimitiveComponent Object Reference") (OtherActor :type "Actor Object Reference") (OtherComp :type "PrimitiveComponent Object Reference") (OtherBodyIndex :type Integer) (bFromSweep :type Boolean) (SweepResult :type "HitResult Structure (by ref)"))
  (bind _aspawn (cast `Pawn` OtherActor))
  ; Checkpoint can only be activated once in lifetime
  (if (`Pawn.IsPlayerControlled` _aspawn)
    (goto _label)))

(event `self.ReceiveTick`
  (params (DeltaSeconds :type "Float (single-precision)"))
  (`self.SetHologramLookAtPlayer`))

(fn `SetHologramColor`
  (params (Color :type "Color Structure"))
  (`MeshComponent.SetColorParameterValueOnMaterials` (`self.HologramMesh`) "Color" (`KismetMathLibrary.Conv_ColorToLinearColor` Color)))

(fn `SetHologramLookAtPlayer`
  (bind _rotpoint (`self.RotPoint`))
  (`SceneComponent.K2_SetWorldRotation` _rotpoint (`KismetMathLibrary.FindLookAtRotation` (`SceneComponent.K2_GetComponentLocation` _rotpoint) (`self.K2_GetActorLocation` (`GameplayStatics.GetPlayerPawn` 0))) false false))

(fn `UserConstructionScript`
  (bind _triggervolume (`self.TriggerVolume`))
  (`SceneComponent.K2_SetRelativeLocationAndRotation` _triggervolume (`self.TriggerLocation`) (`self.TriggerRotation`) false false)
  (`BoxComponent.SetBoxExtent` _triggervolume (`self.TriggerExtent`) true)
  (bind _returnvalue (`|GetDataTableRow` "/Game/_Project/Blueprints/_Core/DataTables/DT_Colors.DT_Colors" "AstroBlue")
    (:`then`
      (set `self.AstroBlue` _returnvalue)
      (bind _returnvalue_2 (`|GetDataTableRow` "/Game/_Project/Blueprints/_Core/DataTables/DT_Colors.DT_Colors" "AstroRed")
        (:`then`
          (bind _output_get (set `self.AstroRed` _returnvalue_2))
          (`self.SetHologramColor` (`.Color_2_4C17D96A4E396D37D036AEA6CFD4D351` (break `/Game/_Project/Blueprints/_Core/Structures/F_Color` _output_get))))))))