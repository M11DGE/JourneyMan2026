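; BP_DoubleDoor is an interactable double door whose two panels swing open in opposite directions and share a material set in the construction script.
; SetDoorState calls OpenDoor or CloseDoor to play or reverse the door timeline and records DoorOpen.
; The timeline's alpha yaws the left and right pivots up to 90 degrees.
; BeginPlay enables player input, but the FlipFlop toggle has no triggering event.
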(event `self.ReceiveBeginPlay`
  (`self.EnableInput` (`GameplayStatics.GetPlayerController` 0)))

(fn `CloseDoor`
  (`TimelineComponent.Reverse` (`self.TL_Door`)))

(fn `OpenDoor`
  (`TimelineComponent.Play` (`self.TL_Door`)))

(fn `SetDoorState`
  (params (BOpen :type Boolean))
  (if BOpen
    (`self.OpenDoor`)
    (set `self.DoorOpen` true)
    (else
      (`self.CloseDoor`)
      (set `self.DoorOpen` false))))

(fn `UserConstructionScript`
  (`|ExecutionSequence`
    (:`then_0`
      (`PrimitiveComponent.SetMaterial` (`self.DooeLeft`) 0 (`self.DoorMaterial`)))
    (:`then_1`
      (`PrimitiveComponent.SetMaterial` (`self.DoorRight`) 0 (`self.DoorMaterial`)))))