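; Lever interactable that, on receiving an attack, sets both BlueDoor and RedDoor states true and retunes two slow zones.
; A timeline spins the cog mesh while new speeds are pushed to overlapping Minecart/Minecraft pawns.
; SlowZone02's update is nested in SlowZone01's loop, so it needs a pawn in the first zone.
; Sphere overlap toggles input and an in-range flag; older alternating-door logic is unconnected.
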(event `self.Sphere.OnComponentBeginOverlap`
  (params (OverlappedComponent :type "PrimitiveComponent Object Reference") (OtherActor :type "Actor Object Reference") (OtherComp :type "PrimitiveComponent Object Reference") (OtherBodyIndex :type Integer) (bFromSweep :type Boolean) (SweepResult :type "HitResult Structure (by ref)"))
  (`self.EnableInput` (`GameplayStatics.GetPlayerController` 0))
  (set `self.BPlayerInRange` true))

(event `/Game/_Project/Blueprints/_Core/Interfaces/BPI_AttackReceiver.OnAttackReceived`
  (params (DamageAmount :type "Float (double-precision)") (KnockbackForce :type "Vector Structure") (Instigator :type "Actor Object Reference") (DamageType :type "/Game/_Project/Blueprints/_Core/Enums/E_DamageType Enum" :default "NewEnumerator0"))
  (bind _slowzone02 (`self.SlowZone02`))
  (bind _slowzone01 (`self.SlowZone01`))
  (`/Game/_Project/Blueprints/Interactables/BP_DoubleDoor.SetDoorState` (`self.BlueDoor`) true)
  (`/Game/_Project/Blueprints/Interactables/BP_DoubleDoor.SetDoorState` (`self.RedDoor`) true)
  (set `/Game/_Project/Blueprints/Interactables/Minecraft/BP_SlowZone.SlowSpeed` 200.0 _slowzone01)
  (`|ExecutionSequence`
    (:`then_0`
      (bind (_direction _spingeargraph) (`Timeline|SpinCogTimeline`)
        (:`Update`
          (`SceneComponent.K2_SetRelativeRotation` (`self.SkeletalMesh`) (`KismetMathLibrary.MakeRotator` 0.0 (`KismetMathLibrary.Lerp` 0.0 360.0 _spingeargraph)) false false))))
    (:`then_1`
      (for _array_element (`self.GetOverlappingActors` (`self.SlowZone01`) "/Game/_Project/Blueprints/Interactables/Minecraft/BP_MinecraftPawnNomarl.BP_MinecraftPawnNomarl_C")
        (bind _asbp_minecraft_pawn_nomarl (cast `/Game/_Project/Blueprints/Interactables/Minecraft/BP_MinecraftPawnNomarl` _array_element))
        (set `FloatingPawnMovement.MaxSpeed` (`/Game/_Project/Blueprints/Interactables/Minecraft/BP_SlowZone.SlowSpeed` _slowzone01) (`/Game/_Project/Blueprints/Interactables/Minecraft/BP_MinecraftPawnNomarl.FloatingPawnMovement` _asbp_minecraft_pawn_nomarl))
        (set `/Game/_Project/Blueprints/Interactables/Minecraft/BP_SlowZone.SlowSpeed` 0.0 _slowzone02)
        (for _array_element_2 (`self.GetOverlappingActors` _slowzone02 "/Game/_Project/Blueprints/Interactables/Minecraft/BP_MinecraftPawnNomarl.BP_MinecraftPawnNomarl_C")
          (bind _asbp_minecraft_pawn_nomarl_2 (cast `/Game/_Project/Blueprints/Interactables/Minecraft/BP_MinecraftPawnNomarl` _array_element_2))
          (set `FloatingPawnMovement.MaxSpeed` (`/Game/_Project/Blueprints/Interactables/Minecraft/BP_SlowZone.SlowSpeed` _slowzone02) (`/Game/_Project/Blueprints/Interactables/Minecraft/BP_MinecraftPawnNomarl.FloatingPawnMovement` _asbp_minecraft_pawn_nomarl_2)))))))

(event `self.Sphere.OnComponentEndOverlap`
  (params (OverlappedComponent :type "PrimitiveComponent Object Reference") (OtherActor :type "Actor Object Reference") (OtherComp :type "PrimitiveComponent Object Reference") (OtherBodyIndex :type Integer))
  (`self.DisableInput` (`GameplayStatics.GetPlayerController` 0))
  (set `self.BPlayerInRange` false))

(fn `UserConstructionScript`)