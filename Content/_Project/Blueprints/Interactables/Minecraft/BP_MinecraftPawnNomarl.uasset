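; Minecraft interactable pawn that drives itself forward along the spline of its ActivePath, with audio playing while it moves.
; Each tick it applies forward movement input, then GetPath turns it toward the spline point nearest a short look-ahead along the local tangent.
; Reaching the last spline point sets Stop, which mutes the audio and destroys the actor after a brief delay.
; An alternative max-speed interpolation is left unconnected.
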(event `self.ReceiveTick`
  (params (DeltaSeconds :type "Float (single-precision)"))
  (if (`self.Stop`)
    (`AudioComponent.SetVolumeMultiplier` (`self.Audio`) 0.0)
    (`KismetSystemLibrary.Delay` 2.0)
    (`self.K2_DestroyActor`)
    (else
      (`AudioComponent.SetVolumeMultiplier` (`self.Audio`) 1.0)
      (`self.AddMovementInput` (`self.GetActorForwardVector`) (`self.Speed`))
      (`self.Get Path`))))

(fn `Get Path`
  (bind _returnvalue (`self.K2_GetActorLocation`))
  (bind _activepath (`self.ActivePath`))
  (bind _spline (`/Game/_Project/Blueprints/Enviroment/BP_RailSplineImproved.Spline` _activepath))
  (`/Engine/EditorBlueprintResources/StandardMacros.IsValid` _activepath
    (:`Is Valid`
      (if (>= (`SplineComponent.FindInputKeyClosestToWorldLocation` _spline (`self.K2_GetActorLocation`)) (- (`SplineComponent.GetNumberOfSplinePoints` _spline) 1))
        (set `self.Stop` true)
        (else
          (`self.K2_SetActorRotation` (`KismetMathLibrary.FindLookAtRotation` _returnvalue (`SplineComponent.FindLocationClosestToWorldLocation` _spline (+ (* (`KismetMathLibrary.Normal` (`SplineComponent.FindTangentClosestToWorldLocation` _spline _returnvalue "World")) 50.0) _returnvalue) "World"))))))))

(fn `UserConstructionScript`)