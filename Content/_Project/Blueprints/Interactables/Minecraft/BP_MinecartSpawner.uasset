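; Minecart spawner actor that keeps a minecart pawn running on an assigned Path.
; StartSpawning spawns a BP_MinecraftPawnNomarl at the spawner's transform with a default controller and the Path as its ActivePath.
; It binds to the cart's OnDestroyed to spawn a replacement each time.
; GM_AstroBot's GameHidden event destroys the current cart, which also fires that respawn binding.
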(event `self.ReceiveBeginPlay`
  (bind _asgm_astor_bot (cast `/Game/_Project/Blueprints/_Core/GM_AstroBot` (`GameplayStatics.GetGameMode`)))
  (add `/Game/_Project/Blueprints/_Core/GM_AstroBot.GameHidden` _asgm_astor_bot (delegate `CustomEvent`)))

(event `CustomEvent`
  (bind _spawnedminecart (`self.SpawnedMinecart`))
  (`/Engine/EditorBlueprintResources/StandardMacros.IsValid` _spawnedminecart
    (:`Is Valid`
      (`self.K2_DestroyActor` _spawnedminecart))))

(event `StartSpawning`
  (`self.SpawnMinecart`)
  (add `self.OnDestroyed` (`self.SpawnedMinecart`) (delegate `OnMinecartDestroyed`)))

(event `OnMinecartDestroyed` :!signature `self.OnDestroyed`
  (params (DestroyedActor :type "Actor Object Reference"))
  (`self.SpawnMinecart`)
  (add `self.OnDestroyed` (`self.SpawnedMinecart`) (delegate `OnMinecartDestroyed`)))

(fn `SpawnMinecart`
  (bind _returnvalue (`|SpawnActorFromClass` "/Game/_Project/Blueprints/Interactables/Minecraft/BP_MinecraftPawnNomarl.BP_MinecraftPawnNomarl_C" (`self.GetTransform`) "AlwaysSpawn" "MultiplyWithRoot" null null))
  (bind _output_get (set `self.SpawnedMinecart` _returnvalue))
  (`Pawn.SpawnDefaultController` _output_get)
  (set `/Game/_Project/Blueprints/Interactables/Minecraft/BP_MinecraftPawnNomarl.ActivePath` (`self.Path`) _output_get))

(fn `UserConstructionScript`)