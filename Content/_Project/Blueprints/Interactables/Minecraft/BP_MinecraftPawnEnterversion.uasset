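; Rideable minecart pawn that drives itself along the spline of its active path while it has a rider.
; An overlap volume registers the cart as the player's current minecart and toggles whether it can be entered.
; Each tick it moves forward and turns toward a look-ahead point on the spline, found by projecting along the nearest tangent.
; At the last spline point it stops, silences its audio and allows exit.
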(event `self.ReceiveTick`
  (params (DeltaSeconds :type "Float (single-precision)"))
  (if (`self.HasRider`)
    (if (`self.Stop`)
      (`AudioComponent.Stop` (`self.Audio`))
      (else
        (`self.AddMovementInput` (`self.GetActorForwardVector`) (`self.Speed`))
        (`self.Get Path`)))))

(event `self.EnterRange.OnComponentBeginOverlap`
  (params (OverlappedComponent :type "PrimitiveComponent Object Reference") (OtherActor :type "Actor Object Reference") (OtherComp :type "PrimitiveComponent Object Reference") (OtherBodyIndex :type Integer) (bFromSweep :type Boolean) (SweepResult :type "HitResult Structure (by ref)"))
  (bind _asbp_player (cast `/Game/_Project/Blueprints/Characters/Player/BP_Player` OtherActor))
  (set `/Game/_Project/Blueprints/Characters/Player/BP_Player.CurrentMinecart` self _asbp_player)
  (set `self.CanEnter` true))

(event `self.EnterRange.OnComponentEndOverlap`
  (params (OverlappedComponent :type "PrimitiveComponent Object Reference") (OtherActor :type "Actor Object Reference") (OtherComp :type "PrimitiveComponent Object Reference") (OtherBodyIndex :type Integer))
  (bind _asbp_player (cast `/Game/_Project/Blueprints/Characters/Player/BP_Player` OtherActor))
  (set `/Game/_Project/Blueprints/Characters/Player/BP_Player.CurrentMinecart` null _asbp_player)
  (set `self.CanEnter` false))

(fn `Get Path`
  (bind _returnvalue (`self.K2_GetActorLocation`))
  (bind _activepath (`self.ActivePath`))
  (bind _spline (`/Game/_Project/Blueprints/Interactables/Minecraft/BP_Path.Spline` _activepath))
  (`/Engine/EditorBlueprintResources/StandardMacros.IsValid` _activepath
    (:`Is Valid`
      (if (>= (`SplineComponent.FindInputKeyClosestToWorldLocation` _spline (`self.K2_GetActorLocation`)) (- (`SplineComponent.GetNumberOfSplinePoints` _spline) 1))
        (set `self.Stop` true)
        (set `self.CanExit` true)
        (else
          (`self.K2_SetActorRotation` (`KismetMathLibrary.FindLookAtRotation` _returnvalue (`SplineComponent.FindLocationClosestToWorldLocation` _spline (+ (* (`KismetMathLibrary.Normal` (`SplineComponent.FindTangentClosestToWorldLocation` _spline _returnvalue "World")) 50.0) _returnvalue) "World"))))))))

(fn `UserConstructionScript`)