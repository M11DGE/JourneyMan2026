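; Destructible ice wall that breaks into gibs on impact and changes the movement speed of pawns in its linked Slowzone.
; On impact, it sets the zone's SlowSpeed and copies it to the floating movement max speed of every overlapping BP_MinecraftPawnNomarl.
; The wall destroys itself only when that Slowzone reference is valid.
; Gib spawning is delegated to TurnToGibsFunction, and the attack-received event is empty.
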(event `/Game/_Project/Blueprints/_Core/Interfaces/BPI_Destructible.OnImpact`
  (params (ImpactForce :type "Float (double-precision)") (DamageType :type "/Game/_Project/Blueprints/_Core/Enums/E_DamageType Enum" :default "NewEnumerator0") (ForceOrigin :type "Vector Structure"))
  (bind _slowzone (`self.Slowzone`))
  (`self.TurnToGibsFunction`)
  (`/Engine/EditorBlueprintResources/StandardMacros.IsValid` _slowzone
    (:`Is Valid`
      (set `/Game/_Project/Blueprints/Interactables/Minecraft/BP_SlowZone.SlowSpeed` 200.0 _slowzone)
      (for _array_element (`self.GetOverlappingActors` _slowzone "/Game/_Project/Blueprints/Interactables/Minecraft/BP_MinecraftPawnNomarl.BP_MinecraftPawnNomarl_C")
        (bind _asbp_minecraft_pawn_nomarl (cast `/Game/_Project/Blueprints/Interactables/Minecraft/BP_MinecraftPawnNomarl` _array_element))
        (set `FloatingPawnMovement.MaxSpeed` (`/Game/_Project/Blueprints/Interactables/Minecraft/BP_SlowZone.SlowSpeed` _slowzone) (`/Game/_Project/Blueprints/Interactables/Minecraft/BP_MinecraftPawnNomarl.FloatingPawnMovement` _asbp_minecraft_pawn_nomarl)))
      (`self.K2_DestroyActor`))))

(event `/Game/_Project/Blueprints/_Core/Interfaces/BPI_AttackReceiver.OnAttackReceived`
  (params (DamageAmount :type "Float (double-precision)") (KnockbackForce :type "Vector Structure") (Instigator :type "Actor Object Reference") (DamageType :type "/Game/_Project/Blueprints/_Core/Enums/E_DamageType Enum" :default "NewEnumerator0")))

(fn `UserConstructionScript`
  (`parent.UserConstructionScript`))