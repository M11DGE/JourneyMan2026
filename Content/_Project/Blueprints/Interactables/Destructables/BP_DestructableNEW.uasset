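; Destructible interactable that hides its mesh, disables collision and bursts into gibs the first time it receives an attack.
; A map of offsets to meshes defines the gibs, shifted by actor location without applying rotation or scale.
; Each gib is requested from BP_GibPool with an outward force, hit sound and lifetime.
; The construction script sets the intact mesh and, in debug mode, previews gib placements with a hologram material.
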(event `/Game/_Project/Blueprints/_Core/Interfaces/BPI_AttackReceiver.OnAttackReceived`
  (params (DamageAmount :type "Float (double-precision)") (KnockbackForce :type "Vector Structure") (Instigator :type "Actor Object Reference") (DamageType :type "/Game/_Project/Blueprints/_Core/Enums/E_DamageType Enum" :default "NewEnumerator0"))
  (`self.TurnToGibsFunction`))

(fn `TurnToGibsFunction`
  (bind _vectormeshmap (`self.VectorMeshMap`))
  (bind _sm_breakable (`self.SM_Breakable`))
  (`/Engine/EditorBlueprintResources/StandardMacros.DoOnce` false
    (:`Completed`
      (`SceneComponent.SetVisibility` _sm_breakable false false)
      (`PrimitiveComponent.SetCollisionEnabled` _sm_breakable "NoCollision")
      (`self.VectorMeshMapToGlobal`)
      (bind _returnvalue (`GameplayStatics.GetActorOfClass` "/Game/_Project/Blueprints/_Core/BP_GibPool.BP_GibPool_C"))
      (bind _keys (`BlueprintMapLibrary.Map_Keys` _vectormeshmap))
      (bind _values (`BlueprintMapLibrary.Map_Values` _vectormeshmap))
      (for (_array_element _array_index) _keys
        (`/Game/_Project/Blueprints/_Core/BP_GibPool.TrySpawnGibFromPool` _returnvalue _array_element (* (`KismetMathLibrary.Normal` (- _array_element (`self.K2_GetActorLocation`))) (`self.GibExplosiveForce`)) (`|GetArrayItem` _values _array_index) (`self.GibHitSoundEffect`) (`self.GibLifeTillShrink`))))))

(fn `UserConstructionScript`
  (bind _vectormeshmap (`self.VectorMeshMap`))
  (`StaticMeshComponent.SetStaticMesh` (`self.SM_Breakable`) (`self.MeshIn`))
  (if (`self.bIsDebugGibPostition`)
    (bind _keys (`BlueprintMapLibrary.Map_Keys` _vectormeshmap))
    (for _array_element _keys
      (bind _returnvalue (`AddComponent|NODE_AddStaticMeshComponent-0` :`RelativeTransform` (`KismetMathLibrary.MakeTransform` _array_element)))
      (bind _value (`BlueprintMapLibrary.Map_Find` _vectormeshmap _array_element))
      (`/Engine/EditorBlueprintResources/StandardMacros.IsValid` _value
        (:`Is Valid`
          (`StaticMeshComponent.SetStaticMesh` _returnvalue _value)
          (`PrimitiveComponent.SetMaterial` _returnvalue 0 "/Game/_Project/Art/Materials/MI_Hologram.MI_Hologram"))))))

(fn `VectorMeshMapToGlobal`
  (locals (VectorMeshMap :type "Map of Vector Structure to StaticMesh Object Reference"))
  (bind _vectormeshmap (`self.VectorMeshMap`))
  (bind _keys (`BlueprintMapLibrary.Map_Keys` _vectormeshmap))
  (for _array_element _keys
    (`BlueprintMapLibrary.Map_Add` (`local.VectorMeshMap`) (+ _array_element (`self.K2_GetActorLocation`)) (`BlueprintMapLibrary.Map_Find` _vectormeshmap _array_element)))
  (set `self.VectorMeshMap` (`local.VectorMeshMap`))
  (return))