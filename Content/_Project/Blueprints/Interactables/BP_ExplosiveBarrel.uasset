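; Explosive barrel interactable that detonates when its temperature component reports exceeded heat.
; A DoOnce gate plays ignition audio, waits briefly, then spawns explosion VFX and sound and sends an impact message to every actor overlapping its sphere.
; The barrel is hidden with collision off rather than destroyed, so the game mode's GameHidden event can restore it and re-arm the gate.
; Player overlap input and older destroy/impulse logic are deprecated leftovers.
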(event `self.ReceiveBeginPlay`
  (add `/Game/_Project/Blueprints/_Core/GM_AstroBot.GameHidden` (cast `/Game/_Project/Blueprints/_Core/GM_AstroBot` (`GameplayStatics.GetGameMode`) :!pure true) (delegate `GameHidden`)))

(event `GameHidden`
  (`self.SetInGame` true)
  (goto _label :!via `Reset`))

(event `self.AC_TemperatureComponent.HeatExceeded`
  (`/Engine/EditorBlueprintResources/StandardMacros.DoOnce` false :!label _label
    (:`Completed`
      (`GameplayStatics.PlaySoundAtLocation` "/Game/_Project/Audio/SQ_Ignition.SQ_Ignition" (`self.K2_GetActorLocation`) (struct) 1.0 1.0 0.0 null null null null)
      (`KismetSystemLibrary.Delay` 3.0)
      (`NiagaraFunctionLibrary.SpawnSystemAtLocation` "/Game/_Project/Art/Particles/NS_ExplosionVfx.NS_ExplosionVfx" (`self.K2_GetActorLocation`) (struct) (10.0 10.0 10.0))
      (`GameplayStatics.PlaySoundAtLocation` "/Game/_Project/Audio/SQ_Explosion.SQ_Explosion" (`self.K2_GetActorLocation`) (struct) 1.0 1.0 0.0 null null null null)
      (for _array_element (`PrimitiveComponent.GetOverlappingActors` (`self.Sphere`) null)
        (message `/Game/_Project/Blueprints/_Core/Interfaces/BPI_Destructible.OnImpact` _array_element 10.0 "NewEnumerator0" (`self.K2_GetActorLocation`)))
      (`self.SetInGame` false))))

(event `self.Sphere.OnComponentBeginOverlap`
  (params (OverlappedComponent :type "PrimitiveComponent Object Reference") (OtherActor :type "Actor Object Reference") (OtherComp :type "PrimitiveComponent Object Reference") (OtherBodyIndex :type Integer) (bFromSweep :type Boolean) (SweepResult :type "HitResult Structure (by ref)"))
  ; Deprecated
  (cast `/Game/_Project/Blueprints/Characters/Player/BP_Player` OtherActor)
  (`self.EnableInput` (`GameplayStatics.GetPlayerController` 0))
  (set `self.BPayerInRange` true))

(event `Key|E`
  (params (Key :type "Key Structure"))
  ; Deprecated
  (:`Pressed`
    (if (`self.BPayerInRange`)
      _)))

(event `self.Sphere.OnComponentEndOverlap`
  (params (OverlappedComponent :type "PrimitiveComponent Object Reference") (OtherActor :type "Actor Object Reference") (OtherComp :type "PrimitiveComponent Object Reference") (OtherBodyIndex :type Integer))
  ; Deprecated
  (cast `/Game/_Project/Blueprints/Characters/Player/BP_Player` OtherActor)
  (set `self.BPayerInRange` false))

(fn `SetInGame`
  (params (State :type Boolean))
  (`SceneComponent.SetVisibility` (`self.DefaultSceneRoot`) State true)
  (`self.SetActorEnableCollision` State))

(fn `UserConstructionScript`)