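; Snowball projectile in the Snowman enemy folder that arcs toward a target location and damages the player on contact.
; Construction applies Speed to the projectile movement, then BeginPlay computes a toss velocity toward EndLocation via SuggestProjectileVelocity, with debug drawing enabled.
; Sphere overlap with BP_Player sends an attack message with Damage and destroys the snowball, which otherwise destroys itself after a fixed delay.
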(event `self.ReceiveBeginPlay`
  (bind _tossvelocity (`GameplayStatics.BlueprintSuggestProjectileVelocity` (`self.K2_GetActorLocation`) (`self.EndLocation`) (`self.Speed`) 0.0 "DoNotTrace" 0.0 false true true))
  (set `MovementComponent.Velocity` _tossvelocity (`self.ProjectileMovement`))
  (`KismetSystemLibrary.Delay` 5.0)
  (`self.K2_DestroyActor`))

(event `self.Sphere1.OnComponentBeginOverlap`
  (params (OverlappedComponent :type "PrimitiveComponent Object Reference") (OtherActor :type "Actor Object Reference") (OtherComp :type "PrimitiveComponent Object Reference") (OtherBodyIndex :type Integer) (bFromSweep :type Boolean) (SweepResult :type "HitResult Structure (by ref)"))
  (bind _asbp_player (cast `/Game/_Project/Blueprints/Characters/Player/BP_Player` OtherActor))
  (message `/Game/_Project/Blueprints/_Core/Interfaces/BPI_AttackReceiver.OnAttackReceived` _asbp_player (`self.Damage`) (0.0 0.0 0.0) null "NewEnumerator1")
  (`self.K2_DestroyActor`))

(fn `UserConstructionScript`
  (bind _speed (`self.Speed`))
  (bind _projectilemovement (`self.ProjectileMovement`))
  (set `ProjectileMovementComponent.InitialSpeed` _speed _projectilemovement)
  (set `ProjectileMovementComponent.MaxSpeed` _speed _projectilemovement))