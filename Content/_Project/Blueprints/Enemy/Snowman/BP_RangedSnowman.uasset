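; Ranged snowman enemy that fires a snowball projectile at the player, extending a parent enemy's AI states and attack hooks.
; It faces the player while charging, attacking or stunned, and takes damage from physical or hot hits and excess heat.
; State changes drive timeline scale animations: a shrink pulse that loops ever faster up to a cap while charging, then a swell on attack, with sounds for charge and shot.
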(event `self.ReceiveBeginPlay`
  (`parent.ReceiveBeginPlay`))

(event `self.ReceiveTick`
  (params (DeltaSeconds :type "Float (single-precision)"))
  (bind _ai_state (`self.AI_State`))
  (if (or (`|EnumEquality` _ai_state "NewEnumerator2") (`|EnumEquality` _ai_state "NewEnumerator3") (`|EnumEquality` _ai_state "NewEnumerator7"))
    (`self.FacePlayer`))
  (`parent.ReceiveTick` DeltaSeconds))

(event `/Game/_Project/Blueprints/_Core/Interfaces/BPI_AttackReceiver.OnAttackReceived`
  (params (DamageAmount :type "Float (double-precision)") (KnockbackForce :type "Vector Structure") (Instigator :type "Actor Object Reference") (DamageType :type "/Game/_Project/Blueprints/_Core/Enums/E_DamageType Enum" :default "NewEnumerator0"))
  (switch `/Game/_Project/Blueprints/_Core/Enums/E_AIState` (`self.AI_State`)
    (:`NewEnumerator0`
      _)
    (:`NewEnumerator1`
      _)
    (:`NewEnumerator2`
      _)
    (:`NewEnumerator3`
      _)
    (:`NewEnumerator7`
      _))
  (switch `/Game/_Project/Blueprints/_Core/Enums/E_DamageType` DamageType
    (:`NewEnumerator0`
      _)
    (:`NewEnumerator1`
      _))
  (`self.TakeDamage` (`KismetMathLibrary.FCeil` DamageAmount)))

(event `self.AC_TemperatureComponent.HeatExceeded`
  (`self.TakeDamage` 1))

(event `StartChargeAttackAnimation`
  (bind _output_get (set `self.ChargeAttackAnimPlayrateCurrent` (`self.ChargeAttackAnimPlayrateStart`)))
  (`TimelineComponent.SetPlayRate` (`self.ChargeAttackAnimTimeline`) _output_get)
  (`self.PlayChargeAttackAnim`))

(event `PlayChargeAttackAnim`
  (if (not (`TimelineComponent.IsPlaying` (`self.ChargeAttackAnimTimeline`)))
    (bind (_direction _scalealpha) (`Timeline|ChargeAttackAnimTimeline` :!via `PlayFromStart` :!label _label)
      (:`Update`
        (`SceneComponent.SetRelativeScale3D` (`self.SM_Snowman_Enemy`) (`KismetMathLibrary.VLerp` (1.0 1.0 1.0) (0.95 0.95 0.95) _scalealpha)))
      (:`Finished`
        (bind _output_get (set `self.ChargeAttackAnimPlayrateCurrent` (`KismetMathLibrary.FClamp` (* (`self.ChargeAttackAnimPlayrateCurrent`) 1.5) 1.0 5.0)))
        (`TimelineComponent.SetPlayRate` (`self.ChargeAttackAnimTimeline`) _output_get)
        (`self.PlayChargeAttackAnim`)))))

(event `StopChargeAttackAnim`
  (`SceneComponent.SetRelativeScale3D` (`self.SM_Snowman_Enemy`) (1.0 1.0 1.0))
  (goto _label :!via `Stop`))

(event `StartAttackAnimation`
  (`self.StopChargeAttackAnim`)
  (`TimelineComponent.SetPlayRate` (`self.AttackAnimTimeline`) 2.0)
  (bind (_direction _alpha) (`Timeline|AttackAnimTimeline` :!via `PlayFromStart`)
    (:`Update`
      (`SceneComponent.SetRelativeScale3D` (`self.SM_Snowman_Enemy`) (`KismetMathLibrary.VLerp` (1.0 1.0 1.0) (1.1 1.1 1.1) _alpha)))))

(fn `Attack`
  (`parent.Attack`)
  (`self.FireProjectile`)
  (`GameplayStatics.PlaySoundAtLocation` "/Game/_Project/Audio/SQ_Pop.SQ_Pop" (`self.K2_GetActorLocation`) (struct) 1.0 1.0 0.0 null null null null))

(fn `FireProjectile`
  (`|SpawnActorFromClass` "/Game/_Project/Blueprints/Enemy/Snowman/BP_SnowballProjectile.BP_SnowballProjectile_C" (`SceneComponent.K2_GetComponentToWorld` (`self.Arrow`)) "Undefined" "MultiplyWithRoot" self (`self.ProjectileSpeed`) (`self.K2_GetActorLocation` (`GameplayStatics.GetPlayerPawn` 0)) null))

(fn `PlayChargingAttackSound`
  (`parent.PlayChargingAttackSound`)
  (`GameplayStatics.PlaySoundAtLocation` "/Game/_Project/Audio/SQ_Suck.SQ_Suck" (`self.K2_GetActorLocation`) (struct) 1.0 1.0 0.0 null null null null))

(fn `SetAIState`
  (params (AIState :type "/Game/_Project/Blueprints/_Core/Enums/E_AIState Enum" :default "NewEnumerator0"))
  (`parent.SetAIState` AIState)
  (switch `/Game/_Project/Blueprints/_Core/Enums/E_AIState` AIState
    (:`NewEnumerator2`
      (`self.StartAttackAnimation`))
    (:`NewEnumerator3`
      (`self.StartChargeAttackAnimation`))))

(fn `UserConstructionScript`
  (`parent.UserConstructionScript`))