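; BP_MeleePolarBear is a polar bear enemy with a melee attack, built on a parent class that handles its base behavior.
; Attack runs a single-hit, zero-length box trace matching the HitBox component against one object type and sends an OnAttackReceived interface message to the actor it hits.
; Eye start, tick and end events are forwarded as messages to the ACEye component.
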(event `self.ReceiveBeginPlay`
  (`parent.ReceiveBeginPlay`))

(event `self.ReceiveTick`
  (params (DeltaSeconds :type "Float (single-precision)"))
  (`parent.ReceiveTick` DeltaSeconds))

(event `/Game/Animation_Team_Stuff/EyeSystem/BPI_EyeInterface.EyeEventEnd`
  (message `/Game/Animation_Team_Stuff/EyeSystem/BPI_EyeInterface.EyeEventEnd` (`self.AC_EyeComponent`)))

(event `/Game/Animation_Team_Stuff/EyeSystem/BPI_EyeInterface.EyeEventTick`
  (params (FrameDeltaTime :type "Float (double-precision)"))
  (message `/Game/Animation_Team_Stuff/EyeSystem/BPI_EyeInterface.EyeEventTick` (`self.AC_EyeComponent`) FrameDeltaTime))

(event `/Game/Animation_Team_Stuff/EyeSystem/BPI_EyeInterface.EyeEventStart`
  (params (TotalDuration :type "Float (double-precision)") (EyeAction :type "/Game/Animation_Team_Stuff/EyeSystem/E_EyeActions Enum" :default "NewEnumerator0") (EyeColor :type "LinearColor Structure"))
  (message `/Game/Animation_Team_Stuff/EyeSystem/BPI_EyeInterface.EyeEventStart` (`self.AC_EyeComponent`) TotalDuration EyeAction EyeColor))

(fn `Attack`
  (bind _hitbox (`self.HitBox`))
  (bind _returnvalue (`SceneComponent.K2_GetComponentLocation` _hitbox))
  (bind (_outhit _returnvalue_2) (`KismetSystemLibrary.BoxTraceSingleForObjects` _returnvalue _returnvalue (`BoxComponent.GetScaledBoxExtent` _hitbox) (struct) (`|MakeArray` "ObjectTypeQuery7" :!type "EObjectTypeQuery Enum")))
  (if _returnvalue_2
    (message `/Game/_Project/Blueprints/_Core/Interfaces/BPI_AttackReceiver.OnAttackReceived` (`.HitActor` (`GameplayStatics.BreakHitResult` _outhit)) 1.0 (0.0 0.0 0.0) null "NewEnumerator0")
    (return)))

(fn `UserConstructionScript`
  (`parent.UserConstructionScript`))