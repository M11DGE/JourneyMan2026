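; BP_FlyingCoin is a coin actor that rises on spawn and then turns into a BP_Coin near the player.
; BeginPlay plays a timeline that lerps it from StartLocation to UpLocation, then sets FlyingToPlayer.
; Tick acts only once TargetPlayer is within 50 units: one interpolated step toward the player character, then it spawns BP_Coin and destroys itself.
; StartLocation, UpLocation and TargetPlayer are never assigned in these graphs.
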(event `self.ReceiveBeginPlay`
  (bind (_direction _heightalpha _flyalpha) (`Timeline|TL_FlyUp`)
    (:`Update`
      (`self.K2_SetActorLocation` (`KismetMathLibrary.VLerp` (`self.StartLocation`) (`self.UpLocation`) _heightalpha)))
    (:`Finished`
      (set `self.FlyingToPlayer` true))))

(event `self.ReceiveTick`
  (params (DeltaSeconds :type "Float (single-precision)"))
  (if (`self.FlyingToPlayer`)
    (if (< (`self.GetDistanceTo` (`self.TargetPlayer`)) 50.0)
      (`|ExecutionSequence`
        (:`then_0`
          (`self.K2_SetActorLocation` (`KismetMathLibrary.VInterpTo` (`self.K2_GetActorLocation`) (`self.K2_GetActorLocation` (`GameplayStatics.GetPlayerCharacter` 0)) DeltaSeconds 10.0)))
        (:`then_1`
          (`|SpawnActorFromClass` "/Game/_Project/Blueprints/BP_Coin.BP_Coin_C" (`KismetMathLibrary.Conv_VectorToTransform` (`self.K2_GetActorLocation`)) "Undefined" "MultiplyWithRoot" null null)
          (`self.K2_DestroyActor`))))))

(fn `UserConstructionScript`)