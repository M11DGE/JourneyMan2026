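; Level Sequence director for the end-of-level cinematic, revealing the friend bots the player found.
; GetRefs swaps the player HUD for an animated end-sequence widget, moves the player to a hardcoded location and caches HUD references.
; FindBot events read the HUD's FriendBotsFound map by key index to set per-bot flags.
; Bot events unhide found bots with a frozen-burst Niagara effect, while companion events hide them.
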(event `GetRefs`
  (bind _asbp_player (cast `/Game/_Project/Blueprints/Characters/Player/BP_Player` (`GameplayStatics.GetPlayerCharacter` 0)))
  (bind _output_get (set `self.As BP Player` _asbp_player))
  (`Widget.RemoveFromParent` (`/Game/_Project/Blueprints/_Core/GMC_AstroBotHUD.Player_HUD` (`/Game/_Project/Blueprints/Characters/Player/BP_Player.As GMC Astro Bot HUD` _output_get)))
  (bind _returnvalue (`|CreateWidget` "/Game/_Project/Blueprints/UI/Widgets/End_Sequence/EndSequenceUI.EndSequenceUI_C"))
  (`UserWidget.AddToViewport` _returnvalue 0)
  (`UserWidget.PlayAnimation` _returnvalue (`/Game/_Project/Blueprints/UI/Widgets/End_Sequence/EndSequenceUI.EndSequence` _returnvalue) 0.0 1 "Forward" 1.0 false)
  (`Actor.K2_SetActorLocation` _output_get (-6470.0 2630.0 2493.0) false false)
  (bind _aspc_player (cast `/Game/_Project/Blueprints/_Core/PC_Player` (`GameplayStatics.GetPlayerController` 0)))
  (set `self.Player HUD` (`/Game/_Project/Blueprints/_Core/GMC_AstroBotHUD.Player_HUD` (cast `/Game/_Project/Blueprints/_Core/GMC_AstroBotHUD` (`PlayerController.GetHUD` _aspc_player) :!pure true))))

(event `FindBot1`
  (bind _friendbotsfound (`/Game/_Project/Blueprints/UI/Widgets/Player_HUD/WBP_HUD.FriendBotsFound` (`self.Player HUD`)))
  (bind _keys (`BlueprintMapLibrary.Map_Keys` _friendbotsfound))
  (if (`BlueprintMapLibrary.Map_Find` _friendbotsfound (`|GetArrayItem` _keys))
    (set `self.Bot1Found` true)))

(event `FindBot2`
  (bind _friendbotsfound (`/Game/_Project/Blueprints/UI/Widgets/Player_HUD/WBP_HUD.FriendBotsFound` (`self.Player HUD`)))
  (bind _keys (`BlueprintMapLibrary.Map_Keys` _friendbotsfound))
  (if (`BlueprintMapLibrary.Map_Find` _friendbotsfound (`|GetArrayItem` _keys 1))
    (set `self.Bot2Found` true)))

(event `FindBot3`
  (bind _friendbotsfound (`/Game/_Project/Blueprints/UI/Widgets/Player_HUD/WBP_HUD.FriendBotsFound` (`self.Player HUD`)))
  (bind _keys (`BlueprintMapLibrary.Map_Keys` _friendbotsfound))
  (if (`BlueprintMapLibrary.Map_Find` _friendbotsfound (`|GetArrayItem` _keys 2))
    (set `self.Bot3Found` true)))

(event `Bot1_Event`
  (params (Bot1 :type "SkeletalMeshActor Object Reference"))
  (if (`self.Bot1Found`)
    (`NiagaraFunctionLibrary.SpawnSystemAtLocation` "/Game/_Project/Art/Particles/NS_FrozenBurst.NS_FrozenBurst" (`Actor.K2_GetActorLocation` Bot1))
    (`Actor.SetActorHiddenInGame` Bot1 false)))

(event `Bot2_Event`
  (params (Bot2 :type "SkeletalMeshActor Object Reference"))
  (if (`self.Bot2Found`)
    (`NiagaraFunctionLibrary.SpawnSystemAtLocation` "/Game/_Project/Art/Particles/NS_FrozenBurst.NS_FrozenBurst" (`Actor.K2_GetActorLocation` Bot2))
    (`Actor.SetActorHiddenInGame` Bot2 false)))

(event `Bot3_Event`
  (params (Bot3 :type "SkeletalMeshActor Object Reference"))
  (if (`self.Bot3Found`)
    (`NiagaraFunctionLibrary.SpawnSystemAtLocation` "/Game/_Project/Art/Particles/NS_FrozenBurst.NS_FrozenBurst" (`Actor.K2_GetActorLocation` Bot3))
    (`Actor.SetActorHiddenInGame` Bot3 false)))

(event `Bot3_Event_0`
  (params (Bot3 :type "SkeletalMeshActor Object Reference"))
  (`Actor.SetActorHiddenInGame` Bot3 true))

(event `Bot1_Event_0`
  (params (Bot1 :type "SkeletalMeshActor Object Reference"))
  (`Actor.SetActorHiddenInGame` Bot1 true))

(event `Bot2_Event_0`
  (params (Bot2 :type "SkeletalMeshActor Object Reference"))
  (`Actor.SetActorHiddenInGame` Bot2 true))