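; Camera dolly in the Recording folder that moves a camera along a spline and can steal the player's view on BeginPlay.
; AutoPlay drives it by Timeline at PlayRate, facing sideways, perpendicular to the spline.
; FollowPlayerPosition instead maps the player's height between the spline endpoints' heights (cached only with StealFocus) to spline position each Tick, optionally looking at the player.
; The construction script previews the camera at TestFloat along the spline.
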(event `self.ReceiveBeginPlay`
  (bind _returnvalue (`GameplayStatics.GetPlayerController` 0))
  (bind _spline (`self.Spline`))
  (bind _camera (`self.Camera`))
  (bind _returnvalue_location (`KismetMathLibrary.BreakTransform` (`SplineComponent.GetTransformAtTime` _spline 1.0 "World" false false)))
  (bind _returnvalue_location_2 (`KismetMathLibrary.BreakTransform` (`SplineComponent.GetTransformAtTime` _spline 0.0 "World" false false)))
  (bind (_asbp_player _bsuccess) (cast `/Game/_Project/Blueprints/Characters/Player/BP_Player` (`GameplayStatics.GetPlayerPawn` 0) :!pure true))
  (`|ExecutionSequence`
    (:`then_0`
      (if (`self.StealFocus`)
        (set `self.FirstWorldLocation` _returnvalue_location_2)
        (set `self.LastWorldLocation` _returnvalue_location)
        (set `self.LengthOfSpline` (- _returnvalue_location _returnvalue_location_2))
        (`Controller.SetControlRotation` _returnvalue (`SceneComponent.K2_GetComponentRotation` (`self.Camera`)))
        (`PlayerController.SetViewTargetWithBlend` _returnvalue self 0.0 "VTBlend_Linear" 0.0 false)
        (set `/Game/_Project/Blueprints/Characters/Player/BP_Player.bIsCameraDecoupled` _bsuccess _asbp_player)))
    (:`then_1`
      (if (`self.AutoPlay`)
        (`TimelineComponent.SetPlayRate` (`self.Timeline`) (`self.PlayRate`))
        (bind (_direction _alpha) (`Timeline|Timeline`)
          (:`Update`
            (bind (_returnvalue_location_3 _returnvalue_rotation) (`KismetMathLibrary.BreakTransform` (`SplineComponent.GetTransformAtTime` (`self.Spline`) _alpha "Local" false false)))
            (`SceneComponent.K2_SetRelativeLocation` _camera _returnvalue_location_3 false false)
            (`SceneComponent.K2_SetRelativeRotation` _camera (`KismetMathLibrary.MakeRotFromXZ` (* (`KismetMathLibrary.GetRightVector` _returnvalue_rotation) -1.0) (`KismetMathLibrary.GetUpVector` _returnvalue_rotation)) false false)))))))

(event `self.ReceiveTick`
  (params (DeltaSeconds :type "Float (single-precision)"))
  (bind _camera (`self.Camera`))
  (bind (_firstworldlocation_x _firstworldlocation_y _firstworldlocation_z) (`KismetMathLibrary.BreakVector` (`self.FirstWorldLocation`)))
  (bind (_lastworldlocation_x _lastworldlocation_y _lastworldlocation_z) (`KismetMathLibrary.BreakVector` (`self.LastWorldLocation`)))
  (bind _returnvalue (`self.K2_GetActorLocation` (`GameplayStatics.GetPlayerPawn` 0)))
  (bind _returnvalue_location (`KismetMathLibrary.BreakTransform` (`SplineComponent.GetTransformAtTime` (`self.Spline`) (`KismetMathLibrary.MapRangeClamped` (.z _returnvalue) _firstworldlocation_z _lastworldlocation_z 0.0 1.0) "Local" false false)))
  (if (`self.FollowPlayerPosition`)
    (`SceneComponent.K2_SetRelativeLocation` (`self.Camera`) _returnvalue_location false false)
    (if (`self.LookAtPlayer`)
      (`SceneComponent.K2_SetWorldRotation` _camera (`KismetMathLibrary.FindLookAtRotation` (`SceneComponent.K2_GetComponentLocation` _camera) _returnvalue) false false))))

(fn `UserConstructionScript`
  (bind _returnvalue (`SplineComponent.GetTransformAtTime` (`self.Spline`) (`self.TestFloat`) "Local" false false))
  (`SceneComponent.K2_SetRelativeTransform` (`self.Camera`) (`KismetMathLibrary.SelectTransform` _returnvalue (`KismetMathLibrary.MakeTransform` (.location _returnvalue) (struct) (.scale _returnvalue)) (`self.UseSplineRotation`)) false false))