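; BP_PenguinbackpackPickup is a collectible that gives the player the penguin backpack when they overlap its sphere.
; On overlap it adds an AC_Penguinbackpack component to the player character and calls GetPenguin on the GM_AstroBot game mode.
; It then hides the mesh, disables collision and deactivates its Niagara effect, destroying itself only once that effect reports it has finished.
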(event `self.Sphere.OnComponentBeginOverlap`
  (params (OverlappedComponent :type "PrimitiveComponent Object Reference") (OtherActor :type "Actor Object Reference") (OtherComp :type "PrimitiveComponent Object Reference") (OtherBodyIndex :type Integer) (bFromSweep :type Boolean) (SweepResult :type "HitResult Structure (by ref)"))
  (bind _returnvalue (`GameplayStatics.GetPlayerCharacter` 0))
  (bind _niagara (`self.Niagara`))
  (if (== OtherActor _returnvalue)
    (`|AddComponentByClass` :`self` _returnvalue :`Class` "/Game/_Project/Blueprints/Characters/Player/Weapons/PenguinBackpack/AC_Penguinbackpack.AC_Penguinbackpack_C")
    (`/Game/_Project/Blueprints/_Core/GM_AstroBot.GetPenguin` (cast `/Game/_Project/Blueprints/_Core/GM_AstroBot` (`GameplayStatics.GetGameMode`) :!pure true))
    (`SceneComponent.SetVisibility` (`self.SkeletalMesh`) false false)
    (add `NiagaraComponent.OnSystemFinished` _niagara (delegate `Destroy`))
    (`ActorComponent.Deactivate` _niagara)
    (`PrimitiveComponent.SetCollisionEnabled` (`self.Sphere`) "NoCollision")))

(event `Destroy`
  (params (PSystem :type "NiagaraComponent Object Reference"))
  (`self.K2_DestroyActor`))

(fn `UserConstructionScript`)