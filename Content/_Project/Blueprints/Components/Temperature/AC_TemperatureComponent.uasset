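; Actor component that tracks its owner's temperature and provides optional default freeze and melt effects.
; Hot and Cold changes shift the value within limits, while Absorb recharges the penguin backpack from positive heat and drops to maximum cold; changes broadcast to listeners.
; Freezing spawns a bounds-scaled ice cube with Niagara and sound, grown by a runtime-created timeline that reverses to melt.
; Player void-out resets temperature and ice, with cube destruction delegated to BP_EnemyPawn.
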(event `/Game/_Project/Blueprints/_Core/Interfaces/BPI_Temperature.OnTemperatureChanged`
  (params (Temperature :type "/Game/_Project/Blueprints/_Core/Enums/E_Temperature Enum" :default "NewEnumerator0") (ChangeValue :type Integer) (bIsPenguinBackPack :type Boolean) (PenguinBackPackRef :type "/Game/_Project/Blueprints/Characters/Player/Weapons/PenguinBackpack/AC_Penguinbackpack Object Reference"))
  (set `self.Penguin Back Pack Ref` PenguinBackPackRef)
  (switch `/Game/_Project/Blueprints/_Core/Enums/E_Temperature` Temperature
    (:`NewEnumerator0`
      (`self.SetCurrentTemperature` ChangeValue)
      (`self.CurrentTemperatureChanged` (`self.CurrentTemperature`) :!label _label))
    (:`NewEnumerator1`
      (`self.SetCurrentTemperature` ChangeValue "NewEnumerator1")
      (goto _label))
    (:`NewEnumerator2`
      (if bIsPenguinBackPack
        (if (`self.bCanGiveCharge?`)
          (if (> (`self.CurrentTemperature`) 0)
            (`/Game/_Project/Blueprints/Characters/Player/Weapons/PenguinBackpack/AC_Penguinbackpack.Recharge` (`self.Penguin Back Pack Ref`))
            (`self.SetCurrentTemperature` 0 "NewEnumerator2")
            (goto _label)))))))

(event `ColdExceededEvent`
  (bind _returnvalue (`self.GetOwner`))
  (bind _returnvalue_2 (`Actor.GetComponentByClass` _returnvalue "/Script/Engine.StaticMeshComponent"))
  (bind (_returnvalue_origin _returnvalue_boxextent) (`KismetMathLibrary.BreakBoxSphereBounds` (`StaticMesh.GetBounds` (`self.IceCubeStaticMesh`))))
  (bind (_origin _boxextent) (`KismetSystemLibrary.GetComponentBounds` _returnvalue_2))
  (bind _relativelocation (`SceneComponent.RelativeLocation` _returnvalue_2))
  (bind (_returnvalue_x _returnvalue_y _returnvalue_z) (`KismetMathLibrary.BreakVector` (/ _boxextent _returnvalue_boxextent)))
  (`self.ColdExceeded`)
  (if (`self.bUseDefaultFreeze`)
    (switch `/Game/_Project/Blueprints/_Core/Enums/E_StateChange` (`self.State`)
      (:`NewEnumerator2`
        (`/Engine/EditorBlueprintResources/StandardMacros.IsValid` (`self.NewVar`) :!label _label_2
          (:`Is Valid`
            _)
          (:`Is Not Valid`
            (`self.CreateTimeline` (delegate `TimelineEvent`) (delegate `TimelineFinished`))))
        (`/Engine/EditorBlueprintResources/StandardMacros.IsValid` (`self.IceCube`)
          (:`Is Not Valid`
            (bind _retfloat (`self.ReturnLargestFlaot` (`|MakeArray` _returnvalue_x _returnvalue_y _returnvalue_z)))
            (set `self.DesiredScale` (* (* _retfloat (`self.IceCubeScaleMultiplier`)) (1.0 1.0 1.0)))
            (bind _returnvalue_3 (`|AddComponentByClass` _returnvalue "/Script/Engine.StaticMeshComponent" false (`KismetMathLibrary.MakeTransform` _relativelocation)))
            (bind _output_get (set `self.IceCube` _returnvalue_3))
            (`StaticMeshComponent.SetStaticMesh` _output_get (`self.IceCubeStaticMesh`))
            (`PrimitiveComponent.SetMaterial` _output_get 0 (`self.IceCuberMaterial`))
            (`GameplayStatics.PlaySoundAtLocation` "/Game/_Project/Audio/SQ_Freeze.SQ_Freeze" (`Actor.K2_GetActorLocation` (`self.GetOwner`)) (struct) 1.0 1.0 0.0 null null null null)
            (`TimelineComponent.PlayFromStart` (`self.NewVar`))
            (set `self.bTimelineInProgress` true)
            (set `self.State` "NewEnumerator1")
            (bind _returnvalue_4 (`|AddComponentByClass` (`self.GetOwner`) "/Script/Niagara.NiagaraComponent" false (`KismetMathLibrary.MakeTransform` _relativelocation)))
            (`NiagaraComponent.SetAsset` _returnvalue_4 (`self.NiagaraFrozenSystem`) true)
            (`NiagaraComponent.SetVariableVec3` _returnvalue_4 "Box Size" (* _boxextent 1.1)))))
      (:`NewEnumerator0`
        (goto _label_2))
      (:`NewEnumerator1`
        (if (not (`self.bTimelineInProgress`))
          (goto _label_2))))))

(event `TimelineEvent`
  (params (Output :type "Float (single-precision)"))
  (bind _icecube (`self.IceCube`))
  (`/Engine/EditorBlueprintResources/StandardMacros.IsValid` _icecube
    (:`Is Valid`
      (`SceneComponent.SetRelativeScale3D` _icecube (`KismetMathLibrary.VLerp` (0.0 0.0 0.0) (`self.DesiredScale`) Output)))))

(event `HeatExceededEvent`
  (`self.HeatExceeded`)
  (if (`self.bUseDefaultMelt`)
    (switch `/Game/_Project/Blueprints/_Core/Enums/E_StateChange` (`self.State`)
      (:`NewEnumerator2`
        (`/Engine/EditorBlueprintResources/StandardMacros.IsValid` (`self.IceCube`) :!label _label_3
          (:`Is Valid`
            (`/Engine/EditorBlueprintResources/StandardMacros.IsValid` (`self.NewVar`)
              (:`Is Valid`
                _)
              (:`Is Not Valid`
                (`self.CreateTimeline` (delegate `TimelineEvent`) (delegate `TimelineFinished`))))
            (`TimelineComponent.ReverseFromEnd` (`self.NewVar`))
            (set `self.bTimelineInProgress` true)
            (set `self.State` "NewEnumerator0")
            (`GameplayStatics.PlaySoundAtLocation` "/Game/_Project/Audio/SQ_IceMelt.SQ_IceMelt" (`Actor.K2_GetActorLocation` (`self.GetOwner`)) (struct) 1.0 1.0 0.0 null null null null))))
      (:`NewEnumerator0`
        (if (not (`self.bTimelineInProgress`))
          (goto _label_3)))
      (:`NewEnumerator1`
        (goto _label_3)))))

(event `CreateBindingForVoidOut`
  (params (GameMode :type "/Game/_Project/Blueprints/_Core/GM_AstroBot Object Reference"))
  (add `/Game/_Project/Blueprints/_Core/GM_AstroBot.PlayerVoidOut` GameMode (delegate `Reset`)))

(event `Reset`
  (set `self.CurrentTemperature` 0)
  (`/Engine/EditorBlueprintResources/StandardMacros.IsValid` (`self.IceCube`)
    (:`Is Valid`
      (`/Game/_Project/Blueprints/Enemy/BP_EnemyPawn.DestroyIceCube` (cast `/Game/_Project/Blueprints/Enemy/BP_EnemyPawn` (`self.GetOwner`) :!pure true) (`self.IceCube`) :!label _label_4))
    (:`Is Not Valid`
      _))
  (set `self.IceCube` null)
  (set `self.State` "NewEnumerator2"))

(event `TimelineFinished`
  (bind _icecube (`self.IceCube`))
  (`/Engine/EditorBlueprintResources/StandardMacros.IsValid` _icecube
    (:`Is Valid`
      (if (== (`SceneComponent.RelativeScale3D` _icecube) (0.0 0.0 0.0))
        (goto _label_4)))))

(fn `CreateTimeline`
  (params (InterpFunc :type Delegate) (TimelineFinishedFunc :type Delegate))
  (bind _returnvalue (`|AddComponentByClass` (`self.GetOwner`) "/Script/Engine.TimelineComponent"))
  (bind _output_get (set `self.NewVar` _returnvalue))
  (`TimelineComponent.SetTimelineLength` _output_get 1.0)
  (`TimelineComponent.AddInterpFloat` _output_get "/Game/_Project/Blueprints/_Core/Curves/C_Expo.C_Expo" InterpFunc "Alpha" "AlphaTrack")
  (`TimelineComponent.SetTimelineFinishedFunc` _output_get TimelineFinishedFunc))

(fn `ReturnLargestFlaot`
  (params (ArrayFloats :type "Array of Float (double-precision)"))
  (returns (RetFloat :type "Float (double-precision)"))
  (locals (A :type "Array of Float (double-precision)"))
  (bind _output_get (set `local.A` ArrayFloats))
  (`KismetArrayLibrary.SortFloatArray` _output_get false "Descending")
  (return (`|GetArrayItem` _output_get)))

(fn `SetCurrentTemperature`
  (params (TemperatureChange :type Integer) (Temperature :type "/Game/_Project/Blueprints/_Core/Enums/E_Temperature Enum" :default "NewEnumerator0"))
  (bind _returnvalue (+ TemperatureChange (`self.CurrentTemperature`)))
  (bind _returnvalue_2 (- (`self.CurrentTemperature`) TemperatureChange))
  (switch `/Game/_Project/Blueprints/_Core/Enums/E_Temperature` Temperature
    (:`NewEnumerator0`
      (if (not (> _returnvalue (`self.MaxHeat`)))
        (set `self.CurrentTemperature` _returnvalue)
        (`self.HeatExceededEvent`)))
    (:`NewEnumerator1`
      (if (>= _returnvalue_2 (* (`self.MaxCold`) -1))
        (set `self.CurrentTemperature` _returnvalue_2)
        (`self.ColdExceededEvent` :!label _label)))
    (:`NewEnumerator2`
      (set `self.CurrentTemperature` (* (`self.MaxCold`) -1))
      (goto _label))))