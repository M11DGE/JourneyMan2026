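; Actor component that leaves a trail of BP_TrailOrb actors behind its owner while it is on snow.
; A looping timer, paused at BeginPlay, spawns an orb at the offset owner location once it has moved a minimum distance from the last one.
; Surface change events from a bound AC_FloorCheck unpause the timer on Snow and pause it on any other surface.
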(event `self.ReceiveBeginPlay`
  (set `self.OwnerActor` (`self.GetOwner`))
  (bind _returnvalue (`KismetSystemLibrary.K2_SetTimerDelegate` (delegate `SpawnTrailOrb`) 0.033333 true true))
  (set `self.SpawnTrailTimer` _returnvalue)
  (`self.StopSpawnTrail`))

(event `BindToAC_FloorCheck`
  (params (AC_FloorCheck :type "/Game/_Project/Blueprints/Components/FloorCheck/AC_FloorCheck Object Reference"))
  (add `/Game/_Project/Blueprints/Components/FloorCheck/AC_FloorCheck.SurfaceChanged` AC_FloorCheck (delegate `UpdateSurfaceType`)))

(event `StartSpawnTrail`
  (`KismetSystemLibrary.K2_UnPauseTimerHandle` (`self.SpawnTrailTimer`)))

(event `StopSpawnTrail`
  (`KismetSystemLibrary.K2_PauseTimerHandle` (`self.SpawnTrailTimer`)))

(event `UpdateSurfaceType`
  (params (Surface :type "EPhysicalSurface Enum" :default "SurfaceType_Default"))
  (bind _output_get (set `self.Surface Type` Surface))
  (switch `EPhysicalSurface` _output_get
    (:`SurfaceType_Default`
      (`self.StopSpawnTrail` :!label _label))
    (:`SurfaceType1`
      (`self.StartSpawnTrail`))
    (:`SurfaceType2`
      (goto _label))))

(event `SpawnTrailOrb`
  (bind _trailorbsize (`self.TrailOrbSize`))
  (bind _returnvalue (+ (`Actor.K2_GetActorLocation` (`self.OwnerActor`)) (`self.Offset`)))
  (bind _distance (`self.CheckDistanceFromLastPlacedActor`))
  (if (>= _distance (`self.MinimumDistanceBetweenTrailPoints`))
    (`|SpawnActorFromClass` "/Game/_Project/Blueprints/Components/Trail/BP_TrailOrb.BP_TrailOrb_C" (`KismetMathLibrary.MakeTransform` _returnvalue (struct) (`KismetMathLibrary.MakeVector` _trailorbsize _trailorbsize _trailorbsize)) "Undefined" "MultiplyWithRoot" null (`self.TrailOrbLifetime`) null)
    (set `self.LastPlacedActorLocation` _returnvalue)))

(fn `CheckDistanceFromLastPlacedActor`
  (returns (Distance :type "Float (double-precision)"))
  (return (`KismetMathLibrary.Vector_Distance` (+ (`Actor.K2_GetActorLocation` (`self.OwnerActor`)) (`self.Offset`)) (`self.LastPlacedActorLocation`))))