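; BP_TrailOrb is a trail orb actor that removes itself after a set lifetime unless flagged Persistent.
; On BeginPlay, non-persistent orbs store their starting location and scale, then wait out LifeTime.
; A timeline then interpolates scale between near zero and the original, and location between slightly above the start and the start itself.
; The actor is destroyed when the timeline finishes.
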(event `self.ReceiveBeginPlay`
  (if (not (`self.Persistent`))
    (set `self.StartingLocation` (`self.K2_GetActorLocation`))
    (set `self.StartingScale` (`self.GetActorScale3D`))
    (`KismetSystemLibrary.Delay` (`self.LifeTime`))
    (bind (_direction _alpha) (`Timeline|Timeline`)
      (:`Update`
        (`self.SetActorScale3D` (`KismetMathLibrary.VLerp` (0.01 0.01 0.01) (`self.StartingScale`) _alpha))
        (`self.K2_SetActorLocation` (`KismetMathLibrary.VLerp` (+ (`self.StartingLocation`) (0.0 0.0 25.0)) (`self.StartingLocation`) _alpha)))
      (:`Finished`
        (`self.K2_DestroyActor`)))))

(fn `UserConstructionScript`)