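; Actor component that detects the floor beneath its owner, reporting its surface type and placing a drop shadow decal on it.
; On BeginPlay, if auto-start is enabled, it starts a looping, pausable timer and creates a thin, downward-facing shadow decal attached to the owner.
; Each tick of that timer traces downward, moves the decal to the impact and broadcasts hit and surface-change events, resetting to the default surface on a miss.
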(event `self.ReceiveBeginPlay`
  (bind _owneractor (`self.OwnerActor`))
  (set `self.OwnerActor` (`self.GetOwner`))
  (if (`self.bAutoStartCheck`)
    (`self.StartFloorCheck`)
    ; Drop Shadow
    (bind _returnvalue (`|AddComponentByClass` :`self` _owneractor :`Class` "/Script/Engine.DecalComponent"))
    (bind _output_get (set `self.ShadowDecal` _returnvalue))
    (`DecalComponent.SetDecalMaterial` _output_get "/Game/_Project/Art/Materials/MI_DropShadow.MI_DropShadow")
    (bind _returnvalue_2 (`SceneComponent.K2_AttachToComponent` _output_get (`Actor.RootComponent` _owneractor) "None" "SnapToTarget" "SnapToTarget" "KeepRelative" true))
    (`SceneComponent.K2_SetRelativeRotation` _output_get (struct :`Pitch` -90.0) _returnvalue_2 false)
    ;; Makes the drop shadow thin so it doesn't project on underside of objs
    (`SceneComponent.SetRelativeScale3D` _output_get (0.1 1.0 1.0))))

(event `StartFloorCheck`
  (if (`KismetSystemLibrary.K2_IsValidTimerHandle` (`self.CheckTimer`))
    (`KismetSystemLibrary.K2_UnPauseTimerHandle` (`self.CheckTimer`))
    (else
      (bind _returnvalue (`KismetSystemLibrary.K2_SetTimerDelegate` (delegate `CheckFloor`) (`self.CheckFrequency`) true true))
      (set `self.CheckTimer` _returnvalue))))

(event `StopFloorCheck`
  (if (`KismetSystemLibrary.K2_IsValidTimerHandle` (`self.CheckTimer`))
    (`KismetSystemLibrary.K2_PauseTimerHandle` (`self.CheckTimer`))))

(event `CheckFloor`
  (bind _owneractor (`self.OwnerActor`))
  (bind _returnvalue (`Actor.K2_GetActorLocation` _owneractor))
  (bind (_outhit _returnvalue_2) (`KismetSystemLibrary.LineTraceSingle` _returnvalue (+ _returnvalue (0.0 0.0 -3000.0)) "TraceTypeQuery1" false (`|MakeArray` _owneractor) "Persistent"))
  (if _returnvalue_2
    (bind (_bblockinghit _binitialoverlap _time _distance _location _impactpoint _normal _impactnormal _physmat) (`GameplayStatics.BreakHitResult` _outhit))
    (`SceneComponent.K2_SetWorldLocation` (`self.ShadowDecal`) (+ _impactpoint (0.0 0.0 2.0)) false false)
    (`self.HitFloorSurface` _location)
    (bind _surfacetype (`PhysicalMaterial.SurfaceType` _physmat))
    (if (!= (`KismetSystemLibrary.MakeLiteralByte` (`self.Surface Type`)) (`KismetSystemLibrary.MakeLiteralByte` _surfacetype))
      (bind _output_get (set `self.Surface Type` _surfacetype))
      (`self.SurfaceChanged` _output_get :!label _label))
    (else
      (set `self.Surface Type` "SurfaceType_Default")
      (goto _label))))