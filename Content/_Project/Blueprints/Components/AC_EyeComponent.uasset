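; Actor component that animates a character's eyes through flipbook-style expression sheets on a dynamic "Eyes" material, with optional auto-blinking.
; BeginPlay optionally attaches a visor mesh to the owner, creates the material instance and starts a looping blink timer.
; A runtime-created timeline samples per-action curves to set frame indices for blinks and played actions.
; External start, tick and end eye events override the timeline, setting color and stepping frames over a given duration.
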(event `self.ReceiveBeginPlay`
  (bind _returnvalue (`self.GetOwner`))
  (bind _bcreateeyestaticmesh (`self.bCreateEyeStaticMesh`))
  (bind _returnvalue_2 (select `bool` _bcreateeyestaticmesh :`false` (`Actor.GetComponentByClass` (`self.GetOwner`) "/Script/Engine.SkeletalMeshComponent") :`true` (`self.StaticMeshComp`) :!type "PrimitiveComponent Object Reference"))
  (bind _returnvalue_3 (select `bool` (and (`self.bOverrideDirectSet`) (not _bcreateeyestaticmesh)) :`false` _returnvalue_2 :`true` (cast `PrimitiveComponent` (`self.ComponentToAttachTo`) :!pure true)))
  (bind _returnvalue_4 (`PrimitiveComponent.GetMaterialIndex` _returnvalue_3 "Eyes"))
  (`KismetSystemLibrary.DelayUntilNextTick`)
  (`|ExecutionSequence`
    (:`then_0`
      (if (`self.bCreateEyeStaticMesh`)
        (bind _returnvalue_5 (`|AddComponentByClass` :`self` _returnvalue :`Class` "/Script/Engine.StaticMeshComponent"))
        (bind _output_get (set `self.StaticMeshComp` _returnvalue_5))
        (`PrimitiveComponent.SetCollisionEnabled` _output_get "NoCollision")
        (`StaticMeshComponent.SetStaticMesh` _output_get "/Game/_Project/Art/Meshes/Utility/SM_Visor.SM_Visor")
        (set `self.ComponentToAttachTo` (select `bool` (`self.bOverrideDirectSet`) :`false` (select `bool` (`self.bAttachToStaticMesh`) :`false` (`Actor.GetComponentByClass` _returnvalue "/Script/Engine.SkeletalMeshComponent") :`true` (`Actor.GetComponentByClass` _returnvalue "/Script/Engine.StaticMeshComponent") :!type "SceneComponent Object Reference") :`true` (`self.ComponentToAttachTo`)))
        (`KismetSystemLibrary.DelayUntilNextTick`)
        (bind _componenttoattachto (`self.ComponentToAttachTo`)
          (:`then`
            (`SceneComponent.K2_AttachToComponent` _output_get _componenttoattachto (`self.SocketName`) "SnapToTarget" "SnapToTarget" "SnapToTarget" true))
          (:`else`
            (`KismetSystemLibrary.PrintString` "Component to attach to is invalid")))))
    (:`then_1`
      (bind _returnvalue_6 (`PrimitiveComponent.CreateDynamicMaterialInstance` _returnvalue_3 _returnvalue_4 (`PrimitiveComponent.GetMaterial` _returnvalue_3 _returnvalue_4) "MI_Eyes"))
      (bind _output_get_2 (set `self.EyesMaterial` _returnvalue_6))
      (`PrimitiveComponent.SetMaterial` _returnvalue_2 _returnvalue_4 _output_get_2)
      (`PrimitiveComponent.SetMaterial` _returnvalue_3 _returnvalue_4 _output_get_2))
    (:`then_2`
      (if (`self.bAutoBlink`)
        (bind _returnvalue_7 (`|AddComponentByClass` (`self.GetOwner`) "/Script/Engine.TimelineComponent"))
        (bind _output_get_3 (set `self.NewVar` _returnvalue_7))
        (`TimelineComponent.SetTimelineFinishedFunc` _output_get_3 (delegate `TimelineFinished`))
        (`TimelineComponent.AddInterpFloat` _output_get_3 "/Game/_Project/Blueprints/_Core/Curves/C_Linear.C_Linear" (delegate `LinearTimeline`) "Linear" "Alpha")
        (`TimelineComponent.SetPlayRate` _output_get_3 4.0 :!label _label)
        (set `self.BlinkCurve` (`.Curve_6_FB71DE164F7428E78F7E00B5901DEFBC` (break `/Game/Animation_Team_Stuff/EyeSystem/F_EyeAction` (`BlueprintMapLibrary.Map_Find` (`self.ActionMap`) "NewEnumerator1"))))
        (bind _returnvalue_8 (`KismetSystemLibrary.K2_SetTimerDelegate` (delegate `TriggerBlink`) (`self.TimeBetweenBlinks`) true false 1.0 0.5))
        (set `self.AutoBlinkHandle` _returnvalue_8)
        (set `self.bIsAutoblinkOn` true)))
    (:`then_3`
      (`self.SetEyesDefault`))))

(event `Enable autoblink`
  (goto _label))

(event `/Game/Animation_Team_Stuff/EyeSystem/BPI_EyeInterface.EyeEventEnd`
  (`self.SetEyesDefault`)
  (set `self.bIsAnimEyesPlaying` false))

(event `LinearTimeline`
  (params (Output :type "Float (single-precision)"))
  (bind _returnvalue (select `bool` (`self.bIsAutoblinkOn`) :`false` (`self.CurrentEyeAction`) :`true` "NewEnumerator1"))
  (if (`self.bIsAnimEyesPlaying`)
    (`TimelineComponent.Stop` (`self.NewVar`))
    (else
      (`self.SetEyeExpressionSheet` _returnvalue)
      (`self.SetEyeIndexWithAlpha` (`CurveFloat.GetFloatValue` (`self.BlinkCurve`) Output) _returnvalue))))

(event `/Game/Animation_Team_Stuff/EyeSystem/BPI_EyeInterface.EyeEventTick`
  (params (FrameDeltaTime :type "Float (double-precision)"))
  (`self.SetEyeIndex` FrameDeltaTime))

(event `TriggerBlink`
  (`TimelineComponent.PlayFromStart` (`self.NewVar`)))

(event `PlayEyeAction`
  (params (EyeAction :type "/Game/Animation_Team_Stuff/EyeSystem/E_EyeActions Enum" :default "NewEnumerator0"))
  (bind _newvar (`self.NewVar`))
  (`self.Disable autoblink`)
  (`TimelineComponent.SetPlayRate` _newvar 0.75)
  (bind _output_get (set `self.CurrentEyeAction` EyeAction))
  (`TimelineComponent.PlayFromStart` _newvar)
  (set `self.BlinkCurve` (`.Curve_6_FB71DE164F7428E78F7E00B5901DEFBC` (break `/Game/Animation_Team_Stuff/EyeSystem/F_EyeAction` (`BlueprintMapLibrary.Map_Find` (`self.ActionMap`) _output_get)))))

(event `TimelineFinished`
  (if (not (`self.bIsAutoblinkOn`))
    (`self.SetEyesDefault`)
    (`self.Enable autoblink`)))

(event `Disable autoblink`
  (`KismetSystemLibrary.K2_ClearAndInvalidateTimerHandle` (`self.AutoBlinkHandle`))
  (set `self.bIsAutoblinkOn` false))

(event `/Game/Animation_Team_Stuff/EyeSystem/BPI_EyeInterface.EyeEventStart`
  (params (TotalDuration :type "Float (double-precision)") (EyeAction :type "/Game/Animation_Team_Stuff/EyeSystem/E_EyeActions Enum" :default "NewEnumerator0") (EyeColor :type "LinearColor Structure"))
  (set `self.bIsAnimEyesPlaying` true)
  (bind _output_get (set `self.CurrentEyeAction` EyeAction))
  (bind _output_get_2 (set `self.CurrentEyeColor` EyeColor))
  (set `self.EyeAnimLength` TotalDuration)
  (set `self.CDeltaTime` 0.0)
  (`self.SetEyeExpressionSheet` _output_get)
  (`self.SetEyeIndex` 0.0)
  (`self.SetEyeColor` _output_get_2))

(fn `SetEyeColor`
  (params (Value :type "LinearColor Structure"))
  (bind _eyesmaterial (`self.EyesMaterial`)
    (:`then`
      (`MaterialInstanceDynamic.SetVectorParameterValue` _eyesmaterial "Color" Value))
    (:`else`)))

(fn `SetEyeExpressionSheet`
  (params (InEyeAction :type Byte))
  (bind _eyesmaterial (`self.EyesMaterial`)
    (:`then`
      (`MaterialInstanceDynamic.SetScalarParameterValue` _eyesmaterial "ExpressionSheet" (`KismetMathLibrary.FMax` (- (`KismetMathLibrary.Conv_ByteToDouble` InEyeAction) 1.0))))
    (:`else`)))

(fn `SetEyeIndex`
  (params (DeltaTime :type "Float (double-precision)"))
  (bind _output_get (set `self.CDeltaTime` (+ (`self.CDeltaTime`) DeltaTime)))
  (`self.SetEyeIndexWithAlpha` (`KismetMathLibrary.FClamp` (/ _output_get (`self.EyeAnimLength`)))))

(fn `SetEyeIndexWithAlpha`
  (params (Alpha :type "Float (double-precision)") (EyeAction :type "/Game/Animation_Team_Stuff/EyeSystem/E_EyeActions Enum" :default "NewEnumerator0"))
  (bind _eyesmaterial (`self.EyesMaterial`)
    (:`then`
      (`MaterialInstanceDynamic.SetScalarParameterValue` _eyesmaterial "Index" (`KismetMathLibrary.Conv_IntToDouble` (`KismetMathLibrary.Round` (`KismetMathLibrary.Lerp` 0.0 (`KismetMathLibrary.Conv_IntToDouble` (- (`.NumberOfFrames_2_140769754D65DDF8A9544D859FC0DB33` (break `/Game/Animation_Team_Stuff/EyeSystem/F_EyeAction` (`BlueprintMapLibrary.Map_Find` (`self.ActionMap`) EyeAction))) 1)) Alpha)))))
    (:`else`)))

(fn `SetEyesDefault`
  (`self.SetEyeExpressionSheet` (`self.DefaultExpressionSheet`))
  (bind _eyesmaterial (`self.EyesMaterial`)
    (:`then`
      (`MaterialInstanceDynamic.SetScalarParameterValue` _eyesmaterial "Index" (`KismetMathLibrary.Conv_IntToDouble` (`self.DefaultExpressionIndex`)))
      (`self.SetEyeColor` (`self.DefaultColor`)))
    (:`else`)))