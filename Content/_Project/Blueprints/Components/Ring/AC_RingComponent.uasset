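; Actor component that runs an expanding ring attack on its owner, broadcasting the ring's current distance as it grows.
; Setup adds a hidden, collision-free disk mesh scaled to the radius and a timeline built at runtime, with play rate derived from the ring's completion time.
; Attack waits the ring's delay, then shows the disk and plays the timeline, which drives the material's Size parameter and the distance broadcast until the disk hides on finish.
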(event `Setup`
  (params (FRing :type "/Game/_Project/Blueprints/_Core/Structures/F_Ring Structure") (Radius :type "Float (double-precision)"))
  (bind _returnvalue (* Radius 0.011112))
  (bind _newvar (`self.NewVar`))
  (set `self.Radius` Radius)
  (set `self.FRing` FRing)
  (bind _output_get (set `self.Owner` (`self.GetOwner`)))
  (`|ExecutionSequence`
    (:`then_0`
      (bind _returnvalue_2 (`|AddComponentByClass` :`self` _output_get :`Class` "/Script/Engine.StaticMeshComponent"))
      (`PrimitiveComponent.SetCollisionEnabled` _returnvalue_2 "NoCollision")
      (`StaticMeshComponent.SetStaticMesh` _returnvalue_2 "/Game/_Project/Art/Meshes/Utility/SM_Disk_2.SM_Disk_2")
      (`SceneComponent.SetHiddenInGame` _returnvalue_2 true false)
      (bind _output_get_2 (set `self.StaticMeshComp` _returnvalue_2))
      (`PrimitiveComponent.SetCastShadow` _output_get_2 false)
      (`SceneComponent.SetRelativeScale3D` _returnvalue_2 (`KismetMathLibrary.MakeVector` _returnvalue _returnvalue _returnvalue)))
    (:`then_1`
      (bind _returnvalue_3 (`|AddComponentByClass` _output_get "/Script/Engine.TimelineComponent"))
      (bind _output_get_3 (set `self.NewVar` _returnvalue_3))
      (`TimelineComponent.SetTimelineLength` _output_get_3 1.0)
      (`TimelineComponent.AddInterpFloat` (`self.NewVar`) "/Game/_Project/Blueprints/_Core/Curves/C_LinearInfinite.C_LinearInfinite" (delegate `TimelineTick`) "Alpha" "Alpha")
      (`TimelineComponent.SetPlayRate` _newvar (/ 1.0 (`.TimeToComplete_8_80530CA7492115B97B1D02950721E561` (break `/Game/_Project/Blueprints/_Core/Structures/F_Ring` (`self.FRing`)))))
      (`TimelineComponent.SetTimelineFinishedFunc` _newvar (delegate `TimelineFinish`)))))

(event `TimelineTick`
  (params (Output :type "Float (single-precision)"))
  (`self.RingDistance` (* Output (`self.Radius`)))
  (`MeshComponent.SetScalarParameterValueOnMaterials` (`self.StaticMeshComp`) "Size" Output))

(event `TimelineFinish`
  (`SceneComponent.SetHiddenInGame` (`self.StaticMeshComp`) true false))

(event `Attack`
  (`KismetSystemLibrary.Delay` (`.Delay_7_31B1BDC346FE15E5048934A1C09E98CE` (break `/Game/_Project/Blueprints/_Core/Structures/F_Ring` (`self.FRing`))))
  (`TimelineComponent.PlayFromStart` (`self.NewVar`))
  (`SceneComponent.SetHiddenInGame` (`self.StaticMeshComp`) false false))