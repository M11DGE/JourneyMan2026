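; Explosive barrel that the player ignites with E while inside its Sphere, exploding after a three-second fuse sound delay.
; Sphere overlaps with BP_Player enable input and toggle the in-range flag; input is never disabled on exit.
; The blast spawns effects and sound, then reuses the Sphere's overlaps to explode BP_DestructibleWall actors and launch BP_IceCube meshes horizontally away with a mass-independent impulse, before destroying itself.
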(event `self.ReceiveBeginPlay`)

(event `self.Sphere.OnComponentBeginOverlap`
  (params (OverlappedComponent :type "PrimitiveComponent Object Reference") (OtherActor :type "Actor Object Reference") (OtherComp :type "PrimitiveComponent Object Reference") (OtherBodyIndex :type Integer) (bFromSweep :type Boolean) (SweepResult :type "HitResult Structure (by ref)"))
  (cast `/Game/_Project/Blueprints/Characters/Player/BP_Player` OtherActor)
  (`self.EnableInput` (`GameplayStatics.GetPlayerController` 0))
  (set `self.BPayerInRange` true))

(event `Key|E`
  (params (Key :type "Key Structure"))
  (:`Pressed`
    (if (`self.BPayerInRange`)
      (`GameplayStatics.PlaySoundAtLocation` "/Game/_Project/Blueprints/Ignition_sound.Ignition_sound" (`self.K2_GetActorLocation`) (struct) 1.0 1.0 0.0 null null null null)
      (`KismetSystemLibrary.Delay` 3.0)
      (`NiagaraFunctionLibrary.SpawnSystemAtLocation` "/Game/_Project/Blueprints/S1mpleExplosion.S1mpleExplosion" (`self.K2_GetActorLocation`) (struct) (10.0 10.0 10.0))
      (`GameplayStatics.PlaySoundAtLocation` "/Game/_Project/Audio/ExplosionSound.ExplosionSound" (`self.K2_GetActorLocation`) (struct) 1.0 1.0 0.0 null null null null)
      (`|ExecutionSequence`
        (:`then_0`
          (for _array_element (`PrimitiveComponent.GetOverlappingActors` (`self.Sphere`) null)
            (`|ExecutionSequence`
              (:`then_0`
                (bind _asbp_destructible_wall (cast `/Game/_Project/Blueprints/BP_DestructibleWall` _array_element))
                (`/Game/_Project/Blueprints/BP_DestructibleWall.Explode` _asbp_destructible_wall))
              (:`then_1`
                (bind _asbp_ice_cube (cast `/Game/_Project/Blueprints/BP_IceCube` _array_element))
                (`PrimitiveComponent.AddImpulse` (`/Game/_Project/Blueprints/BP_IceCube.IceCubeMesh` _asbp_ice_cube) (* (`KismetMathLibrary.Normal` (`KismetMathLibrary.MakeVector` (.x (- (`self.K2_GetActorLocation` _asbp_ice_cube) (`self.K2_GetActorLocation`))) (.y (- (`self.K2_GetActorLocation` _asbp_ice_cube) (`self.K2_GetActorLocation`))))) 3000.0) "None" true))))
          (`self.K2_DestroyActor`))))))

(event `self.Sphere.OnComponentEndOverlap`
  (params (OverlappedComponent :type "PrimitiveComponent Object Reference") (OtherActor :type "Actor Object Reference") (OtherComp :type "PrimitiveComponent Object Reference") (OtherBodyIndex :type Integer))
  (cast `/Game/_Project/Blueprints/Characters/Player/BP_Player` OtherActor)
  (`self.EnableInput` (`GameplayStatics.GetPlayerController` 0))
  (set `self.BPayerInRange` false))

(fn `UserConstructionScript`)