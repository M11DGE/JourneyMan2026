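; BP_Destructable_Chest is a chest that breaks open and spawns coins when attacked.
; On the first attack received, gated by a DoOnce, it plays explosion and chest-break sounds and hides the lid mesh with its collision disabled.
; It then has BPCoinSpawnComponent spawn the configured number of coins and forwards the attack to the parent handler, so later hits do neither.
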(event `/Game/_Project/Blueprints/_Core/Interfaces/BPI_AttackReceiver.OnAttackReceived`
  (params (DamageAmount :type "Float (double-precision)") (KnockbackForce :type "Vector Structure") (Instigator :type "Actor Object Reference") (DamageType :type "/Game/_Project/Blueprints/_Core/Enums/E_DamageType Enum" :default "NewEnumerator0"))
  (bind _returnvalue (`self.K2_GetActorLocation`))
  (bind _sm_itembox_lid (`self.SM_ItemBox_Lid`))
  (`/Engine/EditorBlueprintResources/StandardMacros.DoOnce` false
    (:`Completed`
      (`GameplayStatics.PlaySoundAtLocation` "/Game/_Project/Audio/SQ_Explosion.SQ_Explosion" _returnvalue (struct) 0.4 1.0 0.0 null null null null)
      (`GameplayStatics.PlaySoundAtLocation` "/Game/_Project/Audio/SQ_ChestBreak.SQ_ChestBreak" _returnvalue (struct) 1.0 1.0 0.0 null null null null)
      (`SceneComponent.SetVisibility` _sm_itembox_lid false false)
      (`PrimitiveComponent.SetCollisionEnabled` _sm_itembox_lid "NoCollision")
      (`/Game/_Project/Blueprints/Components/BP_CoinSpawnComponent.SpawnCoins` (`self.BP_CoinSpawnComponent`) (`self.Number Of Coin`))
      (`parent.OnAttackReceived` DamageAmount KnockbackForce Instigator DamageType))))

(fn `UserConstructionScript`
  (`parent.UserConstructionScript`))