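; BP_IcePillar is an ice pillar with a snow top that travels between two points while bobbing vertically.
; The construction script picks both meshes, with SnowTopType setting the base and IcePillarType the top, and previews the starting position.
; MovementTimeline ping-pongs X/Y along a selectable linear or cubic curve, while a separately offset BobTimeline drives Z through a curve.
; Tick applies the combined relative location.
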(event `self.ReceiveBeginPlay`
  (bind _returnvalue (/ (`self.BobHeightChange`) 2.0))
  (switch `/Game/_Project/Blueprints/_Core/Enums/E_Curves` (`self.TimelineCurve`)
    (:`NewEnumerator0`
      (set `self.FloatCurve` "/Game/_Project/Blueprints/_Core/Curves/C_LinearPingPong.C_LinearPingPong"))
    (:`NewEnumerator1`
      (set `self.FloatCurve` "/Game/_Project/Blueprints/_Core/Curves/C_Cubic.C_Cubic")))
  (`TimelineComponent.SetTimelineLength` (`self.MovementTimeline`) (`self.TimeToReachDestination`))
  (`|ExecutionSequence`
    (:`then_0`
      (bind (_direction _alpha) (`Timeline|MovementTimeline` :`NewTime` (`self.StartingTime`) :!via `SetNewTime` :!label _label)
        (:`Update`
          (set `self.Direction` _direction)
          (bind (_returnvalue_x _returnvalue_y) (`KismetMathLibrary.BreakVector` (`KismetMathLibrary.VLerp` (`self.StartVector`) (`self.DestinationVector`) (`CurveFloat.GetFloatValue` (`self.FloatCurve`) (/ _alpha (`self.TimeToReachDestination`))))))
          (set `self.X` _returnvalue_x)
          (set `self.Y` _returnvalue_y))
        (:`Finished`
          (`self.Loop`))))
    (:`then_1`
      (goto _label))
    (:`then_2`
      (`|ExecutionSequence`
        (:`then_0`
          (bind (_direction_2 _alpha_2) (`Timeline|BobTimeline` :`NewTime` (`self.BobOffset`) :!via `SetNewTime` :!label _label_2)
            (:`Update`
              (set `self.Z` (`KismetMathLibrary.Lerp` (* _returnvalue -1.0) _returnvalue (`CurveFloat.GetFloatValue` (`self.ParabCurve`) (/ _alpha_2 (`self.CompleteBobTime`))))))))
        (:`then_1`
          (`TimelineComponent.SetTimelineLength` (`self.BobTimeline`) (`self.CompleteBobTime`))
          (goto _label_2))))))

(event `Loop`
  (switch `ETimelineDirection` (`self.Direction`)
    (:`Forward`
      (goto _label :!via `ReverseFromEnd`))
    (:`Backward`
      (goto _label :!via `PlayFromStart`))))

(event `self.ReceiveTick`
  (params (DeltaSeconds :type "Float (single-precision)"))
  (`SceneComponent.K2_SetRelativeLocation` (`self.IcePillar`) (`KismetMathLibrary.MakeVector` (`self.X`) (`self.Y`) (`self.Z`)) false false))

(fn `UserConstructionScript`
  (switch `/Game/_Project/Blueprints/_Core/Enums/E_Number` (`self.SnowTopType`)
    (:`NewEnumerator0`
      (set `self.IcePillarMesh` "/Game/_Project/Art/Meshes/Platforms/SM_IcePillar_Base_1.SM_IcePillar_Base_1"))
    (:`NewEnumerator1`
      (set `self.IcePillarMesh` "/Game/_Project/Art/Meshes/Platforms/SM_IcePillar_Base_2.SM_IcePillar_Base_2"))
    (:`NewEnumerator2`
      (set `self.IcePillarMesh` "/Game/_Project/Art/Meshes/Platforms/SM_IcePillar_Base_3.SM_IcePillar_Base_3")))
  (switch `/Game/_Project/Blueprints/_Core/Enums/E_Number` (`self.IcePillarType`)
    (:`NewEnumerator0`
      (set `self.SnowTopMesh` "/Game/_Project/Art/Meshes/Platforms/SM_IcePillar_Top_1.SM_IcePillar_Top_1"))
    (:`NewEnumerator1`
      (set `self.SnowTopMesh` "/Game/_Project/Art/Meshes/Platforms/SM_IcePillar_Top_2.SM_IcePillar_Top_2"))
    (:`NewEnumerator2`
      (set `self.SnowTopMesh` "/Game/_Project/Art/Meshes/Platforms/SM_IcePillar_Top_3.SM_IcePillar_Top_3")))
  (`StaticMeshComponent.SetStaticMesh` (`self.IcePillar`) (`self.IcePillarMesh`))
  (`StaticMeshComponent.SetStaticMesh` (`self.SnowTop`) (`self.SnowTopMesh`))
  (`SceneComponent.K2_SetRelativeTransform` (`self.SnowTop`) (`self.SnowTopRelativeTransform`) false false)
  (`SceneComponent.K2_SetRelativeLocation` (`self.IcePillar`) (`KismetMathLibrary.VLerp` (`self.StartVector`) (`self.DestinationVector`) (`KismetMathLibrary.FClamp` (/ (`self.StartingTime`) (`self.TimeToReachDestination`)))) false false))