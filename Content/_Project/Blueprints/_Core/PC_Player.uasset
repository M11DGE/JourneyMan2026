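; Player controller for an Astro Bot-style game that manages which Enhanced Input mapping contexts are active.
; On BeginPlay it adds the movement context and binds to GM_AstorBot game mode events for void-out, game hidden and penguin backpack pickup.
; Void-out removes both the movement and backpack contexts, and the game-hidden event restores movement.
; A pickup flag makes that restore also re-add the backpack context.
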(event `self.ReceiveBeginPlay`
  (bind _asgm_astor_bot (cast `/Game/_Project/Blueprints/GM_AstorBot` (`GameplayStatics.GetGameMode`) :!pure true))
  (add `/Game/_Project/Blueprints/GM_AstorBot.PlayerVoidOut` _asgm_astor_bot (delegate `DisablePlayerInput`))
  (add `/Game/_Project/Blueprints/GM_AstorBot.GameHidden` _asgm_astor_bot (delegate `EnablePlayerInput`))
  (add `/Game/_Project/Blueprints/GM_AstorBot.PlayerPickedUpPenguinBackpack` _asgm_astor_bot (delegate `PlayerGainedPGBP`))
  (`EnhancedInputSubsystemInterface.AddMappingContext` (subsystem `EnhancedInputLocalPlayerSubsystem`) "/Game/_Project/Blueprints/_Core/MappingContexts/IMC_AstroBotMovement.IMC_AstroBotMovement" 0 (struct)))

(event `PlayerGainedPGBP`
  (set `self.bPlayerhasPGBP` true))

(event `EnablePlayerInput`
  (bind _returnvalue (subsystem `EnhancedInputLocalPlayerSubsystem`))
  (`EnhancedInputSubsystemInterface.AddMappingContext` _returnvalue "/Game/_Project/Blueprints/_Core/MappingContexts/IMC_AstroBotMovement.IMC_AstroBotMovement" 0 (struct))
  (if (`self.bPlayerhasPGBP`)
    (`EnhancedInputSubsystemInterface.AddMappingContext` _returnvalue "/Game/_Project/Blueprints/Characters/Player/Weapons/PenguinBackpack/Input/IMC_PenguinBackpack.IMC_PenguinBackpack" 0 (struct))))

(event `DisablePlayerInput`
  (bind _returnvalue (subsystem `EnhancedInputLocalPlayerSubsystem`))
  (`EnhancedInputSubsystemInterface.RemoveMappingContext` _returnvalue "/Game/_Project/Blueprints/_Core/MappingContexts/IMC_AstroBotMovement.IMC_AstroBotMovement" (struct))
  (`EnhancedInputSubsystemInterface.RemoveMappingContext` _returnvalue "/Game/_Project/Blueprints/Characters/Player/Weapons/PenguinBackpack/Input/IMC_PenguinBackpack.IMC_PenguinBackpack" (struct)))

(fn `UserConstructionScript`)