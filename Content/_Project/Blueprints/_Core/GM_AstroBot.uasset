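; Game mode for an Astro Bot style game that handles player death, checkpoint respawns and collectable pickups.
; On player death it broadcasts a void-out, waits, signals game hidden, then teleports the player to the saved checkpoint.
; Checkpoint updates clear the map, keeping only the latest ID and transform.
; Coin, friend, puzzle and penguin pickups update the HUD, with event dispatchers announcing coins, the penguin backpack and checkpoint hits.
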(event `self.ReceiveBeginPlay`
  (bind _asgmc_astro_bot_hud (cast `/Game/_Project/Blueprints/_Core/GMC_AstroBotHUD` (`PlayerController.GetHUD` (`GameplayStatics.GetPlayerController` 0))))
  (set `self.As GMC Astro Bot HUD` _asgmc_astro_bot_hud)
  (bind _asbp_player (cast `/Game/_Project/Blueprints/Characters/Player/BP_Player` (`GameplayStatics.GetPlayerCharacter` 0)))
  (add `/Game/_Project/Blueprints/Characters/Player/BP_Player.OnPlayerDeath` _asbp_player (delegate `HandlePlayerDeath`)))

(event `HandlePlayerDeath`
  (`self.PlayerVoidOut`)
  (`KismetSystemLibrary.Delay` (`self.VoidOutDuration`))
  (`self.GameHidden`)
  (`self.MovePlayerToCheckpoint`))

(event `/Game/_Project/Blueprints/_Core/Interfaces/BPI_Collectable.AddCollectable`
  (params (Type :type "/Game/_Project/Blueprints/_Core/Enums/E_Collectable Enum" :default "NewEnumerator0") (Value :type Integer))
  (bind _as_gmc_astro_bot_hud (`self.As GMC Astro Bot HUD`))
  (switch `/Game/_Project/Blueprints/_Core/Enums/E_Collectable` Type
    (:`NewEnumerator0`
      (`/Game/_Project/Blueprints/_Core/GMC_AstroBotHUD.Coins!` _as_gmc_astro_bot_hud Value)
      (`self.PlayerGetCoin`))
    (:`NewEnumerator1`
      (`/Game/_Project/Blueprints/_Core/GMC_AstroBotHUD.Which Friend Bot?` _as_gmc_astro_bot_hud Value)
      (`/Engine/EditorBlueprintResources/StandardMacros.IncrementInt` (`self.Friend Bots`)))
    (:`NewEnumerator2`
      (`/Game/_Project/Blueprints/_Core/GMC_AstroBotHUD.Which Puzzle Piece?` _as_gmc_astro_bot_hud Value)
      (`/Engine/EditorBlueprintResources/StandardMacros.IncrementInt` (`self.Puzzle Pieces`)))))

(event `GetPenguin`
  (`self.PlayerPickedUpPenguinBackpack`)
  (`/Game/_Project/Blueprints/_Core/GMC_AstroBotHUD.Tutorial` (`self.As GMC Astro Bot HUD`)))

(fn `MovePlayerToCheckpoint`
  (bind _activecheckpointmap (`self.ActiveCheckPointMap`))
  (bind _keys (`BlueprintMapLibrary.Map_Keys` _activecheckpointmap))
  (`self.K2_SetActorTransform` (`GameplayStatics.GetPlayerCharacter` 0) (`BlueprintMapLibrary.Map_Find` _activecheckpointmap (`|GetArrayItem` _keys (`KismetArrayLibrary.Array_LastIndex` _keys))) false false))

(fn `UpdateActiveCheckpoint`
  (params (NewTransform :type "Transform Structure") (CheckpointID :type Integer))
  (returns (bWasAccepted :type Boolean))
  (bind _activecheckpointmap (`self.ActiveCheckPointMap`))
  (`self.CheckPointHit` CheckpointID)
  (`BlueprintMapLibrary.Map_Clear` _activecheckpointmap)
  (`BlueprintMapLibrary.Map_Add` _activecheckpointmap CheckpointID NewTransform)
  (return true))

(fn `UserConstructionScript`)