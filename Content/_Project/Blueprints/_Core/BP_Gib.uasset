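; BP_Gib is a pooled physics debris actor that starts disabled and registers itself with its pool on BeginPlay.
; SpawnFromPool sets the mesh, enables physics and collision, then applies a directional impulse plus a randomly offset radial impulse, both mass-independent, for scatter.
; After the given lifetime, it hides, disables physics and collision, resets its mesh transform and returns to the pool.
; It stores any supplied sound effect but does not play it here.
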(event `self.ReceiveBeginPlay`
  (`self.ReturnToPool`))

(event `SpawnFromPool`
  (params (Location :type "Vector Structure") (StaticMesh :type "StaticMesh Object Reference") (DirectionalForce :type "Vector Structure") (LifeTime :type "Float (double-precision)") (SoundEffect :type "SoundCue Object Reference"))
  (bind _staticmesh (`self.StaticMesh`))
  (`|ExecutionSequence`
    (:`then_0`
      (`StaticMeshComponent.SetStaticMesh` (`self.StaticMesh`) StaticMesh)
      (`self.Enable/Disable` true Location)
      (`PrimitiveComponent.AddImpulse` _staticmesh DirectionalForce "None" true)
      (`PrimitiveComponent.AddRadialImpulse` _staticmesh (+ (`self.K2_GetActorLocation`) (`KismetMathLibrary.RandomUnitVector`)) 25.0 1000.0 "RIF_Constant" true)
      (`self.LifeTime` LifeTime))
    (:`then_1`
      (`/Engine/EditorBlueprintResources/StandardMacros.IsValid` SoundEffect
        (:`Is Valid`
          (set `self.Sound Effect` SoundEffect))))))

(event `ReturnToPool`
  (`self.Enable/Disable` false)
  (set `self.Sound Effect` null)
  (`/Game/_Project/Blueprints/_Core/BP_GibPool.ReturnGibToPool` (`self.Pool`) self))

(event `LifeTime`
  (params (LifeTime :type "Float (double-precision)"))
  (`KismetSystemLibrary.Delay` LifeTime)
  (`self.ReturnToPool`))

(fn `Enable/Disable`
  (params (bIsEnabled :type Boolean) (Location :type "Vector Structure"))
  (bind _staticmesh (`self.StaticMesh`))
  (`self.K2_SetActorLocation` Location false true)
  (`PrimitiveComponent.SetSimulatePhysics` (`self.StaticMesh`) bIsEnabled)
  (`SceneComponent.SetHiddenInGame` (`self.DefaultSceneRoot`) (not bIsEnabled) true)
  (if bIsEnabled
    (`PrimitiveComponent.SetCollisionEnabled` _staticmesh "QueryAndPhysics")
    (else
      (`PrimitiveComponent.SetCollisionEnabled` _staticmesh "NoCollision")
      (`SceneComponent.K2_SetRelativeLocationAndRotation` :`self` (`self.StaticMesh`)))))

(fn `UserConstructionScript`)