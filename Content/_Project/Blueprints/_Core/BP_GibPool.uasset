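; Object pool actor that pre-spawns BP_Gib actors at BeginPlay and reuses them for gib requests.
; A gib-to-bool map tracks use: requests activate the first free gib with position, velocity, mesh, sound and lifetime, and returns mark it free.
; With none free, it spawns another, or at the maximum recycles a random gib despite the FreeOldGib name, then retries recursively.
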(event `self.ReceiveBeginPlay`
  (`self.SpawnNewGibs` (`self.InitiallyGeneratedGibs`)))

(event `RequestGib`
  (params (Position :type "Vector Structure") (Velocity :type "Vector Structure") (StaticMesh :type "StaticMesh Object Reference") (SoundCue :type "SoundCue Object Reference") (LifeTime :type "Float (double-precision)"))
  (`self.TrySpawnGibFromPool` Position Velocity StaticMesh SoundCue LifeTime))

(event `ReturnGibToPool`
  (params (Gib :type "/Game/_Project/Blueprints/_Core/BP_Gib Object Reference"))
  (`BlueprintMapLibrary.Map_Add` (`self.MapOfGibsWithBools`) Gib))

(fn `FreeOldGib`
  (bind _keys (`BlueprintMapLibrary.Map_Keys` (`self.MapOfGibsWithBools`)))
  (`/Game/_Project/Blueprints/_Core/BP_Gib.ReturnToPool` (`KismetArrayLibrary.Array_Random` _keys)))

(fn `SpawnNewGibs`
  (params (NumberOfGibs :type Integer))
  (for _ (range 1 (+ NumberOfGibs 1))
    (bind _returnvalue (`|SpawnActorFromClass` "/Game/_Project/Blueprints/_Core/BP_Gib.BP_Gib_C" (`KismetMathLibrary.MakeTransform` (0.0 0.0 0.0)) "Undefined" "MultiplyWithRoot" null self null))
    (`BlueprintMapLibrary.Map_Add` (`self.MapOfGibsWithBools`) _returnvalue)
    (`/Engine/EditorBlueprintResources/StandardMacros.IncrementInt` (`self.CurrentGibs`))))

(fn `TrySpawnGibFromPool`
  (params (Position :type "Vector Structure") (DirectionalForce :type "Vector Structure") (StaticMesh :type "StaticMesh Object Reference") (SoundEffect :type "SoundCue Object Reference") (LifeTime :type "Float (double-precision)"))
  (locals (bFoundFreeGib :type Boolean))
  (bind _mapofgibswithbools (`self.MapOfGibsWithBools`))
  (bind _keys (`BlueprintMapLibrary.Map_Keys` _mapofgibswithbools))
  (bind _values (`BlueprintMapLibrary.Map_Values` _mapofgibswithbools))
  (for (_array_element _array_index) _values
    (if (not _array_element)
      (bind _output (`|GetArrayItem` _keys _array_index))
      (`/Game/_Project/Blueprints/_Core/BP_Gib.SpawnFromPool` _output Position StaticMesh DirectionalForce LifeTime SoundEffect)
      (`BlueprintMapLibrary.Map_Add` (`self.MapOfGibsWithBools`) _output true)
      (set `local.bFoundFreeGib` true)
      (break)))
  (if (`local.bFoundFreeGib`)
    (return)
    (elif (== (`self.CurrentGibs`) (`self.MaxGibs`))
      (`self.FreeOldGib`)
      (`self.TrySpawnGibFromPool` Position DirectionalForce StaticMesh SoundEffect LifeTime)
      (else
        (`self.SpawnNewGibs` 1)
        (`self.TrySpawnGibFromPool` Position DirectionalForce StaticMesh SoundEffect LifeTime)))))

(fn `UserConstructionScript`)