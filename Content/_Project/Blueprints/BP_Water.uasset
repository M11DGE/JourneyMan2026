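; BP_Water is a water volume that makes BP_IceBlock actors float, with its box sized and placed from VolumeTransform at construction.
; Overlap events track blocks inside, scaling their velocity on entry and removing them on exit or when destroyed.
; Each tick applies upward acceleration to tracked blocks, interpolated between surface and depth forces by their Z offset from a water line derived from the volume's bounds.
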(event `self.ReceiveBeginPlay`
  (bind (_origin _boxextent) (`KismetSystemLibrary.GetComponentBounds` (`self.volume`)))
  (set `self.WaterLine` (+ _origin (`KismetMathLibrary.MakeVector` 0.0 (.y _boxextent)))))

(event `self.ReceiveTick`
  (params (DeltaSeconds :type "Float (single-precision)"))
  (for _array_element (`self.IceBlockArray`)
    (bind _iceblock (`/Game/_Project/Blueprints/BP_IceBlock.IceBlock` _array_element))
    (bind (_returnvalue_x _returnvalue_y _returnvalue_z) (`KismetMathLibrary.BreakVector` (- (`self.WaterLine`) (`SceneComponent.K2_GetComponentLocation` _iceblock))))
    (`PrimitiveComponent.AddForce` _iceblock (* (* (`self.BaseValue`) DeltaSeconds) (`KismetMathLibrary.VLerp` (`KismetMathLibrary.MakeVector` 0.0 0.0 (`self.UpwardsForceAtSurface`)) (`KismetMathLibrary.MakeVector` 0.0 0.0 (`self.UpwardsForceAtDepth`)) (`KismetMathLibrary.FClamp` (/ _returnvalue_z 450.0)))) "None" true)))

(event `self.volume.OnComponentBeginOverlap`
  (params (OverlappedComponent :type "PrimitiveComponent Object Reference") (OtherActor :type "Actor Object Reference") (OtherComp :type "PrimitiveComponent Object Reference") (OtherBodyIndex :type Integer) (bFromSweep :type Boolean) (SweepResult :type "HitResult Structure (by ref)"))
  (bind _asbp_ice_block (cast `/Game/_Project/Blueprints/BP_IceBlock` OtherActor))
  (add `/Game/_Project/Blueprints/BP_IceBlock.IceDestory` _asbp_ice_block (delegate `RemoveFromArray`))
  (`KismetArrayLibrary.Array_AddUnique` (`self.IceBlockArray`) _asbp_ice_block)
  (bind _iceblock (`/Game/_Project/Blueprints/BP_IceBlock.IceBlock` _asbp_ice_block))
  (bind _returnvalue (`PrimitiveComponent.GetPhysicsLinearVelocity` _iceblock "None"))
  (`PrimitiveComponent.SetPhysicsLinearVelocity` _iceblock (* _returnvalue (`self.WaterHitVelocityReductionPercent`)) false "None"))

(event `RemoveFromArray`
  (params (IceBlock :type "/Game/_Project/Blueprints/BP_IceBlock Object Reference"))
  (`KismetArrayLibrary.Array_RemoveItem` (`self.IceBlockArray`) IceBlock)
  (remove `/Game/_Project/Blueprints/BP_IceBlock.IceDestory` IceBlock (delegate `RemoveFromArray`)))

(event `self.volume.OnComponentEndOverlap`
  (params (OverlappedComponent :type "PrimitiveComponent Object Reference") (OtherActor :type "Actor Object Reference") (OtherComp :type "PrimitiveComponent Object Reference") (OtherBodyIndex :type Integer))
  (bind _asbp_ice_block (cast `/Game/_Project/Blueprints/BP_IceBlock` OtherActor))
  (`self.RemoveFromArray` _asbp_ice_block))

(fn `UserConstructionScript`
  (bind (_volumetransform_location _volumetransform_rotation _volumetransform_scale) (`KismetMathLibrary.BreakTransform` (`self.VolumeTransform`)))
  (bind _volume (`self.volume`))
  (`BoxComponent.SetBoxExtent` _volume (* _volumetransform_scale 32.0) true)
  (`SceneComponent.K2_SetRelativeLocationAndRotation` _volume _volumetransform_location _volumetransform_rotation false false))