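; BP_Lasertrap is a moving laser trap that draws a Niagara beam between its Cubestart and Cubeend components.
; The construction script sets the beam endpoints and feeds the Vectorstart and Vectorend variables to InterpToMovement as relative control points.
; Tick updates both beam endpoints from the cubes' world locations.
; Overlap on Cubeend casts to BP_Player but has no further logic, so it applies no effect.
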(event `self.ReceiveTick`
  (params (DeltaSeconds :type "Float (single-precision)"))
  (`FXSystemComponent.SetVectorParameter` (`self.Niagara`) "Beam Start" (`SceneComponent.K2_GetComponentLocation` (`self.Cubestart`)))
  (`FXSystemComponent.SetVectorParameter` (`self.Niagara`) "Beam End" (`SceneComponent.K2_GetComponentLocation` (`self.Cubeend`))))

(event `self.Cubeend.OnComponentBeginOverlap`
  (params (OverlappedComponent :type "PrimitiveComponent Object Reference") (OtherActor :type "Actor Object Reference") (OtherComp :type "PrimitiveComponent Object Reference") (OtherBodyIndex :type Integer) (bFromSweep :type Boolean) (SweepResult :type "HitResult Structure (by ref)"))
  (cast `/Game/_Project/Blueprints/Characters/Player/BP_Player` OtherActor))

(fn `UserConstructionScript`
  (`FXSystemComponent.SetVectorParameter` (`self.Niagara`) "Beam Start" (`SceneComponent.K2_GetComponentLocation` (`self.Cubestart`)))
  (`FXSystemComponent.SetVectorParameter` (`self.Niagara`) "Beam End" (`SceneComponent.K2_GetComponentLocation` (`self.Cubeend`)))
  (`InterpToMovementComponent.AddControlPointPosition` (`self.InterpToMovement`) (`self.vectorstart`) true)
  (`InterpToMovementComponent.AddControlPointPosition` (`self.InterpToMovement`) (`self.vectorend`) true))