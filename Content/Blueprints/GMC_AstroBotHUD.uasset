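; HUD manager Blueprint for an Astro Bot-style game that relays collectible pickups to the on-screen UI.
; On BeginPlay it creates and adds the HUD, pause menu and settings menu widgets to the viewport, collapsing only the settings menu.
; Custom events forward puzzle piece, coin and friend bot pickups to the HUD.
; It also stores a coin total and counts found friend bots to update the pause menu's tracker.
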(event `self.ReceiveBeginPlay`
  (bind _returnvalue (`GameplayStatics.GetPlayerController` 0))
  (bind _returnvalue_2 (`|CreateWidget` "/Game/_Project/Blueprints/UI/Widgets/Player_HUD/WBP_HUD.WBP_HUD_C" _returnvalue))
  (bind _output_get (set `self.Player_HUD` _returnvalue_2))
  (`UserWidget.AddToViewport` _output_get 0)
  (bind _returnvalue_3 (`|CreateWidget` "/Game/_Project/Blueprints/UI/Widgets/Player_PauseMenu/WBP_PauseMenu.WBP_PauseMenu_C" _returnvalue))
  (bind _output_get_2 (set `self.PauseMenu` _returnvalue_3))
  (`UserWidget.AddToViewport` _output_get_2 1)
  (bind _returnvalue_4 (`|CreateWidget` "/Game/_Project/Blueprints/UI/Widgets/Player_SettingsMenu/WBP_SettingsMenu.WBP_SettingsMenu_C" _returnvalue))
  (bind _output_get_3 (set `self.Settings Menu` _returnvalue_4))
  (`UserWidget.AddToViewport` _output_get_3 0)
  (`Widget.SetVisibility` _output_get_3 "Collapsed"))

(event `Which Puzzle Piece?`
  (params (`Puzzle Piece Val` :type Integer))
  (`/Game/_Project/Blueprints/UI/Widgets/Player_HUD/WBP_HUD.Puzzle Piece has been found` (`self.Player_HUD`) `Puzzle Piece Val`))

(event `Amount of Coins`
  (params (Coins :type Integer))
  (set `self.Coins` Coins))

(event `Coins!`
  (params (`Coins Value` :type Integer))
  (`/Game/_Project/Blueprints/UI/Widgets/Player_HUD/WBP_HUD.Coin Collected` (`self.Player_HUD`)))

(event `Which Friend Bot?`
  (params (`Friend Bot Val` :type Integer))
  (`/Game/_Project/Blueprints/UI/Widgets/Player_HUD/WBP_HUD.Friend Bot has been Found` (`self.Player_HUD`) `Friend Bot Val`)
  (bind _output_get (set `self.FriendBotsFound` (+ (`self.FriendBotsFound`) 1)))
  (`/Game/_Project/Blueprints/UI/Widgets/Player_PauseMenu/WBP_FriendBotTracker.Update Collected` (`/Game/_Project/Blueprints/UI/Widgets/Player_PauseMenu/WBP_PauseMenu.WBP_FriendBotTracker` (`self.PauseMenu`)) _output_get))

(fn `UserConstructionScript`)