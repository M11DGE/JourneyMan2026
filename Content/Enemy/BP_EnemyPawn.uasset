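; Base enemy pawn that spots, chases and attacks the player, takes damage, and drops coins on death.
; Tick runs an AIState machine, with PawnSensing and a pathing-radius sphere triggering chases, and gates and pausable timers pacing AIMoveTo, charge and stun.
; Temperature component events freeze or stun it, while Attack is an empty stub.
; Death hides it below the world, and the game mode's void-out event restores it at its start transform.
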(event `self.ReceiveBeginPlay`
  (bind _asgm_astor_bot (cast `/Game/_Project/Blueprints/GM_AstorBot` (`GameplayStatics.GetGameMode`) :!pure true))
  (set `self.ActorStartingTransform` (`self.GetTransform`))
  (add `/Game/_Project/Blueprints/GM_AstorBot.PlayerVoidOut` _asgm_astor_bot (delegate `Respawn`))
  (`/Game/_Project/Blueprints/Components/Temperature/AC_TemperatureComponent.CreateBindingForVoidOut` (`self.AC_TemperatureComponent`) _asgm_astor_bot))

(event `Respawn`
  (`self.SetAIState` "NewEnumerator6"))

(event `self.PawnSensing.OnSeePawn`
  (params (Pawn :type "Pawn Object Reference"))
  (`/Engine/EditorBlueprintResources/StandardMacros.Gate` false :!label _label
    (:`Exit`
      (bind _asbp_player (cast `/Game/_Project/Blueprints/Characters/Player/BP_Player` Pawn))
      (`/Engine/EditorBlueprintResources/StandardMacros.IsValid` (`self.PlayerReference`)
        (:`Is Valid`
          _)
        (:`Is Not Valid`
          (set `self.PlayerReference` _asbp_player)))
      (`self.DisablePawnSeeing`)
      (`self.PlayerSeen`))))

(event `EnablePawnSeeing`
  (goto _label :!via `Open`))

(event `DisablePawnSeeing`
  (goto _label :!via `Close`))

(event `self.ReceiveTick`
  (params (DeltaSeconds :type "Float (single-precision)"))
  (switch `/Game/Enemy/E_AIState` (`self.AI_State`)
    (:`NewEnumerator1`
      (`self.Chase` (delegate `ChaseEvent`))
      (`self.FacePlayer`))
    (:`NewEnumerator2`
      (`self.Attack`)
      (`self.SetAIState` "NewEnumerator7")
      (`KismetSystemLibrary.Delay` (`self.AttackCooldown`))
      (`self.EnableChargeAttack`))
    (:`NewEnumerator3`
      (`self.ChargeAttack`))
    (:`NewEnumerator7`
      (`self.Create/UnpauseStunnedTimer` (delegate `StunnedEvent`)))))

(event `ChaseEvent`
  (`self.ChaseMacro`))

(event `StunnedEvent`
  (`self.EnableChargeAttack`)
  (`self.SetAIState` "NewEnumerator0"))

(event `ChargeAttack`
  (`/Engine/EditorBlueprintResources/StandardMacros.Gate` false :!label _label_2
    (:`Exit`
      (`self.DisableChargeAttack`)
      (`KismetSystemLibrary.Delay` (`self.AttackChargeTime`))
      (if (`|EnumEquality` (`self.AI_State`) "NewEnumerator3")
        (`self.SetAIState` "NewEnumerator2")
        (else
          (`self.EnableChargeAttack`))))))

(event `EnableChargeAttack`
  (goto _label_2 :!via `Open`))

(event `DisableChargeAttack`
  (goto _label_2 :!via `Close`))

(event `self.AC_TemperatureComponent.ColdExceeded`
  (`self.SetAIState` "NewEnumerator4"))

(event `self.AC_TemperatureComponent.HeatExceeded`
  (`self.SetAIState` "NewEnumerator7"))

(event `self.AI_PathingRange.OnComponentBeginOverlap`
  (params (OverlappedComponent :type "PrimitiveComponent Object Reference") (OtherActor :type "Actor Object Reference") (OtherComp :type "PrimitiveComponent Object Reference") (OtherBodyIndex :type Integer) (bFromSweep :type Boolean) (SweepResult :type "HitResult Structure (by ref)"))
  (cast `/Game/_Project/Blueprints/Characters/Player/BP_Player` OtherActor)
  (`self.PlayerEnteredPathingRadius`))

(event `self.AI_PathingRange.OnComponentEndOverlap`
  (params (OverlappedComponent :type "PrimitiveComponent Object Reference") (OtherActor :type "Actor Object Reference") (OtherComp :type "PrimitiveComponent Object Reference") (OtherBodyIndex :type Integer))
  (cast `/Game/_Project/Blueprints/Characters/Player/BP_Player` OtherActor)
  (`self.PlayerExitedPathingRadius`))

(event `/Game/_Project/Blueprints/_Core/Interfaces/BPI_AttackReceiver.OnAttackReceived`
  (params (DamageAmount :type "Float (double-precision)") (KnockbackForce :type "Vector Structure") (Instigator :type "Actor Object Reference") (DamageType :type "/Game/_Project/Blueprints/_Core/Enums/E_DamageType Enum" :default "NewEnumerator0"))
  (switch `/Game/_Project/Blueprints/_Core/Enums/E_DamageType` DamageType
    (:`NewEnumerator0`
      _)
    (:`NewEnumerator1`
      _))
  (`self.TakeDamage` (`KismetMathLibrary.FCeil` DamageAmount)))

(event `DestroyIceCube`
  (params (IceCubeRef :type "StaticMeshComponent Object Reference"))
  (`ActorComponent.K2_DestroyComponent` IceCubeRef))

(fn `Attack`)

(fn `Chase`
  (params (ChaseEvent :type Delegate))
  (if (> (`self.MaxSpeed`) 0.0)
    (if (`KismetSystemLibrary.K2_IsValidTimerHandle` (`self.ChaseTimerHandle`))
      (if (`KismetSystemLibrary.K2_IsTimerActiveHandle` (`self.ChaseTimerHandle`))
        (return)
        (else
          (`KismetSystemLibrary.K2_UnPauseTimerHandle` (`self.ChaseTimerHandle`))))
      (else
        (bind _returnvalue (`KismetSystemLibrary.K2_SetTimerDelegate` ChaseEvent 0.016667 true true))
        (bind _output_get (set `self.ChaseTimerHandle` _returnvalue))
        (`KismetArrayLibrary.Array_Add` (`self.TimerArray`) _output_get)))
    (return)
    (else
      (`self.SetAIState` "NewEnumerator3")
      (return))))

(fn `Create/UnpauseStunnedTimer`
  (params (Delegate :type Delegate))
  (if (not (`KismetSystemLibrary.K2_IsTimerActiveHandle` (`self.StunnedTimerHandle`)))
    (bind _returnvalue (`KismetSystemLibrary.K2_SetTimerDelegate` Delegate (`self.StunnedDuration`)))
    (bind _output_get (set `self.StunnedTimerHandle` _returnvalue))
    (`KismetArrayLibrary.Array_AddUnique` (`self.TimerArray`) _output_get)
    (return)))

(fn `DebugAttackRadius`
  (bind _returnvalue (`AddComponent|NODE_AddSphereComponent-1`))
  (`ShapeComponent.SetLineThickness` _returnvalue 4.0)
  (`SphereComponent.SetSphereRadius` _returnvalue (`self.AttackRadius`) false)
  (`PrimitiveComponent.SetCollisionEnabled` _returnvalue "NoCollision")
  (return))

(fn `Die`
  (`/Game/_Project/Blueprints/Components/BP_CoinSpawnComponent.SpawnCoins` (`self.BP_CoinSpawnComponent`) (`self.CoinValue`))
  (`self.SetAIState` "NewEnumerator5")
  (`self.AIDie`))

(fn `FacePlayer`
  (bind (_returnvalue_roll _returnvalue_pitch _returnvalue_yaw) (`KismetMathLibrary.BreakRotator` (`KismetMathLibrary.FindLookAtRotation` (`SceneComponent.K2_GetComponentLocation` (`self.DefaultSceneRoot`)) (`self.K2_GetActorLocation` (`self.PlayerReference`)))))
  (`/Engine/EditorBlueprintResources/StandardMacros.IsValid` (`self.PlayerReference`)
    (:`Is Valid`
      (`SceneComponent.K2_SetWorldRotation` (`self.DefaultSceneRoot`) (`KismetMathLibrary.MakeRotator` 0.0 0.0 _returnvalue_yaw) false false))))

(fn `Idle`
  (if (`self.bCanRoam`)
    _))

(fn `PauseAllTimers`
  (for _array_element (`self.TimerArray`)
    (`KismetSystemLibrary.K2_PauseTimerHandle` _array_element))
  (return))

(fn `PlayerEnteredPathingRadius`
  (set `self.bPlayerInPathingRadius` true)
  (return))

(fn `PlayerExitedPathingRadius`
  (set `self.bPlayerInPathingRadius` false)
  (if (!= (`self.AI_State`) (`KismetSystemLibrary.MakeLiteralByte` (enumliteral `/Game/Enemy/E_AIState` "NewEnumerator4")))
    (`self.SetAIState` "NewEnumerator0")
    (return)))

(fn `PlayerSeen`
  (`self.AISeenPlayer`)
  (if (`self.bPlayerInPathingRadius`)
    (`self.SetAIState` "NewEnumerator1")
    (else
      (`self.SetAIState` "NewEnumerator0")))
  (return))

(fn `SetAIState`
  (params (AIState :type "/Game/Enemy/E_AIState Enum" :default "NewEnumerator0"))
  (`self.PauseAllTimers`)
  (`MovementComponent.StopMovementImmediately` (`self.FloatingPawnMovement`))
  (bind _output_get (set `self.AI_State` AIState))
  (`KismetSystemLibrary.PrintString` (`|GetEnumeratorNameAsString` _output_get))
  (switch `/Game/Enemy/E_AIState` _output_get
    (:`NewEnumerator0`
      (`self.EnablePawnSeeing`)
      (if (`self.bPlayerInPathingRadius`)
        (`self.SetAIState` "NewEnumerator1"))
      (return))
    (:`NewEnumerator1`
      (return))
    (:`NewEnumerator2`
      (return))
    (:`NewEnumerator3`
      (return))
    (:`NewEnumerator4`
      (`self.DisablePawnSeeing`))
    (:`NewEnumerator5`
      (`self.ToggleInGame` false)
      (return))
    (:`NewEnumerator6`
      (`self.ToggleInGame` true)
      (return))
    (:`NewEnumerator7`
      (return))))

(fn `TakeDamage`
  (params (Amount :type Integer))
  (bind _currenthealth (`self.CurrentHealth`))
  (if (> _currenthealth 0)
    (bind _output_get (set `self.CurrentHealth` (- _currenthealth Amount)))
    (if (== _output_get 0)
      (`self.Die`))
    (`self.AITakeDamage`)))

(fn `ToggleInGame`
  (params (bIsInGame :type Boolean))
  (`|ExecutionSequence`
    (:`then_0`
      (`PawnSensingComponent.SetSensingUpdatesEnabled` (`self.PawnSensing`) bIsInGame))
    (:`then_1`
      (`self.SetActorHiddenInGame` (not bIsInGame)))
    (:`then_2`
      (set `PrimitiveComponent.bGenerateOverlapEvents` bIsInGame (`self.AI_PathingRange`)))
    (:`then_3`
      (if bIsInGame
        (`self.K2_SetActorTransform` (`self.ActorStartingTransform`) false true)
        (set `self.CurrentHealth` (`self.MaxHealth`))
        (else
          (`self.K2_SetActorLocation` (0.0 0.0 -10000.0) false true))))))

(fn `UserConstructionScript`
  (bind _ai_pathfindingcapsule (`self.AI_PathfindingCapsule`))
  (bind _ai_pathfindingcapsule_2 (`self.AI_PathfindingCapsule`))
  (bind _capsulehalfheight (`CapsuleComponent.CapsuleHalfHeight` _ai_pathfindingcapsule))
  (`PawnSensingComponent.SetPeripheralVisionAngle` (`self.PawnSensing`) (`self.PeripheralVisionAngle`))
  (`SphereComponent.SetSphereRadius` (`self.AI_PathingRange`) (`self.MaxPathingRadius`) false)
  (set `FloatingPawnMovement.MaxSpeed` (`self.MaxSpeed`) (`self.FloatingPawnMovement`))
  (set `self.CurrentHealth` (`self.MaxHealth`))
  (if (`self.bDebugAttackRadius`)
    (`self.DebugAttackRadius`)
    (`SceneComponent.K2_SetRelativeLocation` _ai_pathfindingcapsule (`KismetMathLibrary.MakeVector` 0.0 0.0 _capsulehalfheight) false false)
    (`SceneComponent.K2_SetRelativeLocation` (`self.AI_PathingRange`) (`KismetMathLibrary.MakeVector` 0.0 0.0 _capsulehalfheight) false false)
    (set `NavMovementComponent.NavAgentProps` (make `NavAgentProperties` (`CapsuleComponent.CapsuleRadius` _ai_pathfindingcapsule_2) (* (`CapsuleComponent.CapsuleHalfHeight` _ai_pathfindingcapsule_2) 2.0) -1.0 0.5 "None" false false true) (`self.FloatingPawnMovement`))
    (`SceneComponent.SetVisibility` (`self.AI_PathfindingCapsule`) (`self.bDebugPathfindingCapsule`) false)))