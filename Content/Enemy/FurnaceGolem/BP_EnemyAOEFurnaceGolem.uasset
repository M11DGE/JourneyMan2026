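; Furnace golem enemy whose area attack fires a set of rings around it that knock the player back.
; BeginPlay spawns one AC_RingComponent per RingArray entry, sized to the RingExtent sphere, and Attack triggers them all.
; RingExtent overlaps track the player; each ring's distance event does a small sphere trace at that distance toward the player.
; Hits receive an attack message with outward knockback, so only players standing on the ring are struck.
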(event `self.ReceiveBeginPlay`
  (`parent.ReceiveBeginPlay`)
  (for _array_element (`self.RingArray`)
    (bind _returnvalue (`|AddComponentByClass` "/Game/_Project/Blueprints/Components/Ring/AC_RingComponent.AC_RingComponent_C"))
    (`KismetArrayLibrary.Array_Add` (`self.RingComponentArray`) _returnvalue)
    (`/Game/_Project/Blueprints/Components/Ring/AC_RingComponent.Setup` _returnvalue _array_element (`SphereComponent.SphereRadius` (`self.RingExtent`)))
    (add `/Game/_Project/Blueprints/Components/Ring/AC_RingComponent.RingDistance` _returnvalue (delegate `CheckPlayerDistanceAgainstRingDistance`))))

(event `self.ReceiveTick`
  (params (DeltaSeconds :type "Float (single-precision)"))
  (`parent.ReceiveTick` DeltaSeconds))

(event `AttackSequence`
  (for _array_element (`self.RingComponentArray`)
    (`/Game/_Project/Blueprints/Components/Ring/AC_RingComponent.Attack` _array_element)))

(event `CheckPlayerDistanceAgainstRingDistance`
  (params (Distance :type "Float (double-precision)"))
  (bind _returnvalue (`self.K2_GetActorLocation`))
  (bind _as_bp_player (`self.As BP Player`))
  (bind _returnvalue_2 (`KismetMathLibrary.Vector_Normal2D` (- (`self.K2_GetActorLocation` _as_bp_player) _returnvalue)))
  (bind (_returnvalue_x _returnvalue_y) (`KismetMathLibrary.BreakVector` (* Distance _returnvalue_2)))
  (bind _returnvalue_3 (+ (`KismetMathLibrary.MakeVector` _returnvalue_x _returnvalue_y) _returnvalue (0.0 0.0 0.0)))
  (`/Engine/EditorBlueprintResources/StandardMacros.IsValid` _as_bp_player
    (:`Is Valid`
      (bind (_outhits _returnvalue_4) (`KismetSystemLibrary.SphereTraceMultiByProfile` _returnvalue_3 _returnvalue_3 10.0 "Player"))
      (if _returnvalue_4
        (for _array_element _outhits
          (message `/Game/_Project/Blueprints/_Core/Interfaces/BPI_AttackReceiver.OnAttackReceived` (`.HitActor` (`GameplayStatics.BreakHitResult` _array_element)) 1.0 (* _returnvalue_2 1000.0) null "NewEnumerator1"))))))

(event `self.RingExtent.OnComponentBeginOverlap`
  (params (OverlappedComponent :type "PrimitiveComponent Object Reference") (OtherActor :type "Actor Object Reference") (OtherComp :type "PrimitiveComponent Object Reference") (OtherBodyIndex :type Integer) (bFromSweep :type Boolean) (SweepResult :type "HitResult Structure (by ref)"))
  (bind _asbp_player (cast `/Game/_Project/Blueprints/Characters/Player/BP_Player` OtherActor))
  (set `self.As BP Player` _asbp_player))

(event `self.RingExtent.OnComponentEndOverlap`
  (params (OverlappedComponent :type "PrimitiveComponent Object Reference") (OtherActor :type "Actor Object Reference") (OtherComp :type "PrimitiveComponent Object Reference") (OtherBodyIndex :type Integer))
  (cast `/Game/_Project/Blueprints/Characters/Player/BP_Player` OtherActor)
  (set `self.As BP Player` null))

(fn `Attack`
  (`self.AttackSequence`))

(fn `UserConstructionScript`
  (`parent.UserConstructionScript`)
  (`SphereComponent.SetSphereRadius` (`self.RingExtent`) (`self.RingExtentRadius`) true)
  (`SceneComponent.SetHiddenInGame` (`self.RingExtent`) (not (`self.bDebugRingExtentRadius`)) false))