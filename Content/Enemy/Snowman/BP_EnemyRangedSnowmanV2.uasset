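; BP_EnemyRangedSnowmanV2 is a ranged snowman enemy that attacks the player by throwing snowballs.
; It extends a parent Blueprint's behavior, adding a per-tick turn to face the player in three of the AI states.
; Its Attack override calls the parent, then spawns a snowball projectile at the Arrow component's transform, passing it a speed and the player's current location as the end point.
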(event `self.ReceiveBeginPlay`
  (`parent.ReceiveBeginPlay`))

(event `self.ReceiveTick`
  (params (DeltaSeconds :type "Float (single-precision)"))
  (bind _ai_state (`self.AI_State`))
  (if (or (`|EnumEquality` _ai_state "NewEnumerator2") (`|EnumEquality` _ai_state "NewEnumerator3") (`|EnumEquality` _ai_state "NewEnumerator7"))
    (`self.FacePlayer`))
  (`parent.ReceiveTick` DeltaSeconds))

(fn `Attack`
  (`parent.Attack`)
  (`self.FireProjectile`))

(fn `FireProjectile`
  (`|SpawnActorFromClass` "/Game/Enemy/Snowman/BP_SnowballProjectile.BP_SnowballProjectile_C" (`SceneComponent.K2_GetComponentToWorld` (`self.Arrow`)) "Undefined" "MultiplyWithRoot" null (`self.ProjectileSpeed`) (`self.K2_GetActorLocation` (`GameplayStatics.GetPlayerPawn` 0)) null))

(fn `UserConstructionScript`
  (`parent.UserConstructionScript`))