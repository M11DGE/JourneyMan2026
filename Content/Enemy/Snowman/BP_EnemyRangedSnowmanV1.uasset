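; BP_EnemyRangedSnowmanV1 is a ranged snowman enemy that shoots snowballs at the player.
; RangeArea overlaps with BP_Player toggle InRange.
; While Activated and in range, Tick yaws the root and fully rotates the Gun toward the player's mesh.
; A cooldown Delay on Tick paces firing, rechecking range before spawning BP_SnowballProjectile at the Arrow's transform.
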(event `self.RangeArea.OnComponentBeginOverlap`
  (params (OverlappedComponent :type "PrimitiveComponent Object Reference") (OtherActor :type "Actor Object Reference") (OtherComp :type "PrimitiveComponent Object Reference") (OtherBodyIndex :type Integer) (bFromSweep :type Boolean) (SweepResult :type "HitResult Structure (by ref)"))
  (cast `/Game/_Project/Blueprints/Characters/Player/BP_Player` OtherActor)
  (set `self.InRange?` true))

(event `self.ReceiveTick`
  (params (DeltaSeconds :type "Float (single-precision)"))
  (bind (_returnvalue_roll _returnvalue_pitch _returnvalue_yaw) (`KismetMathLibrary.BreakRotator` (`KismetMathLibrary.FindLookAtRotation` (`SceneComponent.K2_GetComponentLocation` (`self.DefaultSceneRoot`)) (`SceneComponent.K2_GetComponentLocation` (`Character.Mesh` (`GameplayStatics.GetPlayerCharacter` 0))))))
  (if (`self.Activated`)
    (if (`self.InRange?`)
      (`|ExecutionSequence`
        (:`then_0`
          (bind _output_get (set `/Game/Enemy/BP_BaseEnemy.AttackCooldown` (`self.Attack Cooldown`) (`self.BP_BaseEnemy`)))
          (`KismetSystemLibrary.Delay` _output_get)
          (if (`self.InRange?`)
            (`self.FireProjectile`)))
        (:`then_1`
          (`SceneComponent.K2_SetWorldRotation` (`self.DefaultSceneRoot`) (`KismetMathLibrary.MakeRotator` 0.0 0.0 _returnvalue_yaw) false false)
          (`SceneComponent.K2_SetWorldRotation` (`self.Gun`) (`KismetMathLibrary.MakeRotator` _returnvalue_roll _returnvalue_pitch _returnvalue_yaw) false false))))))

(event `self.RangeArea.OnComponentEndOverlap`
  (params (OverlappedComponent :type "PrimitiveComponent Object Reference") (OtherActor :type "Actor Object Reference") (OtherComp :type "PrimitiveComponent Object Reference") (OtherBodyIndex :type Integer))
  (cast `/Game/_Project/Blueprints/Characters/Player/BP_Player` OtherActor)
  (set `self.InRange?` false))

(fn `FireProjectile`
  (`|SpawnActorFromClass` "/Game/Enemy/Snowman/BP_SnowballProjectile.BP_SnowballProjectile_C" (`SceneComponent.K2_GetComponentToWorld` (`self.Arrow`)) "Undefined" "MultiplyWithRoot" null null))

(fn `StunCheck`)

(fn `UserConstructionScript`)